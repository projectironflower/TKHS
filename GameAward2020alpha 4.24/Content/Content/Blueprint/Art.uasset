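; Actor Blueprint for a nine-piece artwork that shows memory pieces according to the player's cleared-stage items.
; On BeginPlay it copies ClearItemStruct from MyGameInstance, then SetMemoryPiece hides all pieces and reveals pairs based on the first flag of each of Stage01 to Stage04.
; The middle piece, Art05, stays hidden until the GetLastPiece event makes it visible.
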(event Custom|GetLastPiece
  (Rendering|SetVisibility (Variables|Default|GetArt05) true false))

(event EventBeginPlay
  ;[1 1 1] GameInstanceを変数に取得
  (bind _asmy_game_instance (Utilities|Casting|CastToMyGameInstance (Game|GetGameInstance)))
  (bind _output_get (Variables|Default|SetGameInstance _asmy_game_instance))
  (Variables|Default|SetClearItemStruct (Variables|/Game/Content/GameInstance/MyGameInstance.MyGameInstance_C|GetClearItem_Struct _output_get))
  (Utilities|SetMemoryPiece))

(event Collision|EventActorBeginOverlap
  (params (OtherActor :type Actor%20Object%20Reference)))

(event EventTick
  (params (DeltaSeconds :type Float%20%28single-precision%29)))

(fn ConstructionScript)