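; Press machine hazard that repeatedly slams down and rises, dealing heavy damage to the player it hits while falling.
; Tick drives a four-state cycle of top wait, fall, bottom wait and rise, moving the mesh at speeds normalized to 60 fps.
; Box overlap with a step-up-able non-player component ends the fall with a sound.
; Start activates it after a delay; Stop deactivates it, and Reset returns the mesh to the actor's location.
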(event OnComponentBeginOverlap(Box)
  (params (OverlappedComponent :type Primitive%20Component%20Object%20Reference) (OtherActor :type Actor%20Object%20Reference) (OtherComp :type Primitive%20Component%20Object%20Reference) (OtherBodyIndex :type Integer) (bFromSweep :type Boolean) (SweepResult :type Hit%20Result%20Structure%20%28by%20ref%29))
  (bind (_asplayer_bp _bsuccess) (Utilities|Casting|CastToPlayer_BP OtherActor))
  (if (== (Variables|Default|GetStateNumber) 1)
    (if _bsuccess
      (Default|Damage _asplayer_bp 1e+02)
      (elif (Class|PrimitiveComponent|CanCharacterStepUp OtherComp _asplayer_bp)
        (Variables|Default|SetStateNumber 2)
        (Audio|PlaySoundatLocation "/Game/Content/Sound/SE/SE_Press.SE_Press" (Transformation|GetWorldLocation (Variables|Default|GetStaticMesh)) "0, 0, 0" 1.0 1.0 0.1 "/Game/Content/Sound/SoundAttenuation.SoundAttenuation" 0 0)))))

(event Custom|Stop
  (Variables|Default|SetIsActive false)
  (Default|CallOnSwitched))

(event Custom|Reset
  (bind _staticmesh (Variables|Default|GetStaticMesh))
  (Transformation|SetWorldLocation _staticmesh (Transformation|GetActorLocation) false false)
  (if (>= (.Z (Math|Vector|BreakVector (Transformation|GetWorldLocation _staticmesh))) (.Z (Math|Vector|BreakVector (Transformation|GetWorldLocation (Variables|Default|GetDefaultSceneRoot)))))
    (CallFunction|Stop)))

(event Custom|Start
  (Variables|Default|SetIsActive true)
  (Utilities|FlowControl|Delay (Variables|Default|GetStartDelay))
  (Variables|Default|SetDelayFinished true))

(event EventBeginPlay)

(event Collision|EventActorBeginOverlap
  (params (OtherActor :type Actor%20Object%20Reference)))

(event EventTick
  (params (DeltaSeconds :type Float%20%28single-precision%29))
  (if (Variables|Default|GetDelayFinished)
    (if (Variables|Default|GetIsActive)
      (switch int (Variables|Default|GetStateNumber)
        (:0
          (Utilities|Stay))
        (:1
          (Utilities|Fall DeltaSeconds))
        (:2
          (Utilities|StayBottom))
        (:3
          (Utilities|Up DeltaSeconds))))))

(fn ConstructionScript)