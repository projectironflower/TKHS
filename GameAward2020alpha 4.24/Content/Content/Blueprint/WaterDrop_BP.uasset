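; WaterDrop_BP is a falling water drop hazard that sends the player back to their starting transform on contact.
; BeginPlay caches the actor's transform and the Player_BP pawn's transform.
; Tick lowers the WaterDrop component by FallSpeed, scaled to a 60 fps baseline, and restores the actor's start transform when the next step would fall below world Z zero.
; The Sphere overlap event teleports any overlapping Player_BP to the cached player transform.
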(event OnComponentBeginOverlap(Sphere)
  (params (OverlappedComponent :type Primitive%20Component%20Object%20Reference) (OtherActor :type Actor%20Object%20Reference) (OtherComp :type Primitive%20Component%20Object%20Reference) (OtherBodyIndex :type Integer) (bFromSweep :type Boolean) (SweepResult :type Hit%20Result%20Structure%20%28by%20ref%29))
  (bind (_asplayer_bp _bsuccess) (Utilities|Casting|CastToPlayer_BP OtherActor))
  (if _bsuccess
    (Transformation|SetActorTransform _asplayer_bp (Variables|Default|GetStartPlayerPos))))

(event EventBeginPlay
  (Variables|Default|SetStartPos (Transformation|GetActorTransform))
  (bind _asplayer_bp (Utilities|Casting|CastToPlayer_BP (Game|Player|GetPlayerPawn 0)))
  (Variables|Default|SetStartPlayerPos (Transformation|GetActorTransform _asplayer_bp)))

(event Collision|EventActorBeginOverlap
  (params (OtherActor :type Actor%20Object%20Reference)))

(event EventTick
  (params (DeltaSeconds :type Float%20%28single-precision%29))
  (bind _returnvalue (/ 1.0 6e+01))
  (bind _waterdrop (Variables|Default|GetWaterDrop))
  (bind _fallspeed (Variables|Default|GetFallSpeed))
  (bind _returnvalue_2 (Transformation|GetWorldLocation _waterdrop))
  (bind _returnvalue_3 (/ DeltaSeconds _returnvalue))
  (bind _returnvalue_4 (* _returnvalue_3 _fallspeed))
  (bind _returnvalue_5 (- (.z _returnvalue_2) _returnvalue_4))
  (Transformation|SetWorldLocation _waterdrop (Math|Vector|MakeVector (.x _returnvalue_2) (.y _returnvalue_2) _returnvalue_5) false false)
  (if (< _returnvalue_5 0.0)
    (Transformation|SetActorTransform (Variables|Default|GetStartPos))))

(fn ConstructionScript)