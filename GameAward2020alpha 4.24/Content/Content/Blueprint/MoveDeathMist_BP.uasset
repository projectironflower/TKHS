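; MoveDeathMist_BP is an actor, apparently a death mist, that creeps toward the PlayerStart reference.
; Each Tick it steps along the normalized direction to PlayerStart, scaled by MoveSpeed and delta time, for frame-rate-independent movement.
; It stops once within 50 units of the target, and moves by SetActorLocation without sweep, so collisions do not block it.
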(event EventBeginPlay)

(event Collision|EventActorBeginOverlap
  (params (OtherActor :type Actor%20Object%20Reference)))

(event EventTick
  (params (DeltaSeconds :type Float%20%28single-precision%29))
  (bind _returnvalue (Transformation|GetActorLocation))
  (bind _playerstart (Variables|Default|GetPlayerStart))
  (bind _returnvalue_2 (Transformation|GetActorLocation _playerstart))
  (bind _returnvalue_3 (- _returnvalue_2 _returnvalue))
  (bind _returnvalue_4 (Math|Vector|VectorLength _returnvalue_3))
  (if (>= _returnvalue_4 5e+01)
    (Transformation|SetActorLocation (+ _returnvalue (* (/ _returnvalue_3 _returnvalue_4) (* DeltaSeconds (Variables|Default|GetMoveSpeed)))) false false)))

(fn ConstructionScript)