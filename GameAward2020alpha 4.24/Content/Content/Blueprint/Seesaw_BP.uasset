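; Seesaw actor whose mesh begins simulating physics when a heavy enough player is inside its trigger box.
; Each Tick it polls the Box for overlapping Player_BP actors and compares each one's CharacterMovement Mass to that player's MaxMass.
; A ratio above MaxMassRatio enables physics simulation on the StaticMesh, and nothing in the graph switches it back off.
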(event EventBeginPlay)

(event Collision|EventActorBeginOverlap
  (params (OtherActor :type Actor%20Object%20Reference)))

(event EventTick
  (params (DeltaSeconds :type Float%20%28single-precision%29))
  (for _array_element (Collision|GetOverlappingActors (Variables|Default|GetBox) "/Game/Content/Blueprint/Player/Player_BP.Player_BP_C" :!class /Script/Engine.PrimitiveComponent)
    (if (.bSuccess (Utilities|Casting|CastToPlayer_BP _array_element))
      (if (> (/ (Variables|/Script/Engine.CharacterMovementComponent|GetMass (Variables|/Script/Engine.Character|GetCharacterMovement (.AsPlayer%20BP (Utilities|Casting|CastToPlayer_BP _array_element)))) (Variables|/Game/Content/Blueprint/Player/Player_BP.Player_BP_C|GetMaxMass (.AsPlayer%20BP (Utilities|Casting|CastToPlayer_BP _array_element)))) (Variables|Default|GetMaxMassRatio))
        (Physics|SetSimulatePhysics (Variables|Default|GetStaticMesh) true)))))

(fn ConstructionScript)