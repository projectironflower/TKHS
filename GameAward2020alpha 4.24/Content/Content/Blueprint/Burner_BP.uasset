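; Burner hazard actor that shuttles back and forth vertically or along Y and burns players inside its flame capsule.
; IsFire, set by Start/Stop or toggled periodically when IsSwitch is on, drives the particles and capsule collision.
; Capsule overlaps flag the player's IsOnFire, and Tick damages flagged players still overlapping.
; Movement, switch timing and damage advance per frame, without delta time.
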(event OnComponentBeginOverlap(Capsule)
  (params (OverlappedComponent :type Primitive%20Component%20Object%20Reference) (OtherActor :type Actor%20Object%20Reference) (OtherComp :type Primitive%20Component%20Object%20Reference) (OtherBodyIndex :type Integer) (bFromSweep :type Boolean) (SweepResult :type Hit%20Result%20Structure%20%28by%20ref%29))
  (bind (_asplayer_bp _bsuccess) (Utilities|Casting|CastToPlayer_BP OtherActor))
  (if _bsuccess
    (Variables|/Game/Content/Blueprint/Player/Player_BP.Player_BP_C|SetIsOnFire _asplayer_bp true)))

(event OnComponentEndOverlap(Capsule)
  (params (OverlappedComponent :type Primitive%20Component%20Object%20Reference) (OtherActor :type Actor%20Object%20Reference) (OtherComp :type Primitive%20Component%20Object%20Reference) (OtherBodyIndex :type Integer))
  (bind (_asplayer_bp _bsuccess) (Utilities|Casting|CastToPlayer_BP OtherActor))
  (if _bsuccess
    (Variables|/Game/Content/Blueprint/Player/Player_BP.Player_BP_C|SetIsOnFire _asplayer_bp false)))

(event Custom|Stop
  (Variables|Default|SetIsFire false))

(event Custom|Start
  (Variables|Default|SetIsFire true))

(event EventBeginPlay
  (if (Variables|Default|GetIsFireReverse)
    (Effects|Components|ParticleSystem|SetTemplate (Variables|Default|GetParticleSystem) "/Game/Content/Particle/P_BurnerReverse.P_BurnerReverse")))

(event Collision|EventActorBeginOverlap
  (params (OtherActor :type Actor%20Object%20Reference)))

(event EventTick
  (params (DeltaSeconds :type Float%20%28single-precision%29))
  (bind _capsule (Variables|Default|GetCapsule))
  (bind _particlesystem (Variables|Default|GetParticleSystem))
  (if (Variables|Default|GetIsFire)
    (Components|Activation|Activate _particlesystem false)
    (Collision|SetCollisionEnabled _capsule "QueryAndPhysics")
    (else
      (Components|Activation|Deactivate _particlesystem)
      (Collision|SetCollisionEnabled _capsule "NoCollision")))
  (if (Variables|Default|GetIsSwitch)
    (CallFunction|SwitchFire))
  (if (Variables|Default|GetIsMoveUp)
    (CallFunction|RoundTripUpDown)
    (else
      (CallFunction|RoundTripLeftRight)))
  (for _array_element (Collision|GetOverlappingActors (Variables|Default|GetCapsule) "/Game/Content/Blueprint/Player/Player_BP.Player_BP_C" :!class /Script/Engine.PrimitiveComponent)
    (bind _asplayer_bp (Utilities|Casting|CastToPlayer_BP _array_element))
    (if (Variables|/Game/Content/Blueprint/Player/Player_BP.Player_BP_C|GetIsOnFire _asplayer_bp)
      (Default|Damage _asplayer_bp (Variables|Default|GetFireDamage)))))

(fn ConstructionScript)

(fn RoundTripLeftRight
  (if (Variables|Default|GetIsMoveReverse)
    (bind _output_get (Variables|Default|SetMoveValue (- (Variables|Default|GetMoveValue) (Variables|Default|GetMoveVelocity))))
    (if (< _output_get 0.0)
      (Variables|Default|SetMoveValue 0.0)
      (Variables|Default|SetIsMoveReverse false)
      (else
        (Transformation|SetActorLocation (- (Transformation|GetActorLocation) (Math|Vector|MakeVector 0.0 (Variables|Default|GetMoveVelocity) 0.0)) false true)
        (return)))
    (else
      (bind _output_get_2 (Variables|Default|SetMoveValue (+ (Variables|Default|GetMoveValue) (Variables|Default|GetMoveVelocity))))
      (if (> _output_get_2 (Variables|Default|GetMoveMax))
        (Variables|Default|SetMoveValue (Variables|Default|GetMoveMax))
        (Variables|Default|SetIsMoveReverse true)
        (else
          (Transformation|SetActorLocation (+ (Transformation|GetActorLocation) (Math|Vector|MakeVector 0.0 (Variables|Default|GetMoveVelocity) 0.0)) false true)
          (return))))))

(fn RoundTripUpDown
  (if (Variables|Default|GetIsMoveReverse)
    (bind _output_get (Variables|Default|SetMoveValue (- (Variables|Default|GetMoveValue) (Variables|Default|GetMoveVelocity))))
    (if (< _output_get 0.0)
      (Variables|Default|SetMoveValue 0.0)
      (Variables|Default|SetIsMoveReverse false)
      (else
        (Transformation|SetActorLocation (- (Transformation|GetActorLocation) (Math|Vector|MakeVector 0.0 0.0 (Variables|Default|GetMoveVelocity))) false true)
        (return)))
    (else
      (bind _output_get_2 (Variables|Default|SetMoveValue (+ (Variables|Default|GetMoveValue) (Variables|Default|GetMoveVelocity))))
      (if (> _output_get_2 (Variables|Default|GetMoveMax))
        (Variables|Default|SetMoveValue (Variables|Default|GetMoveMax))
        (Variables|Default|SetIsMoveReverse true)
        (else
          (Transformation|SetActorLocation (+ (Transformation|GetActorLocation) (Math|Vector|MakeVector 0.0 0.0 (Variables|Default|GetMoveVelocity))) false true)
          (return))))))

(fn SwitchFire
  (bind _output_get (Variables|Default|SetElapseTime (+ (Variables|Default|GetElapseTime) 1.0)))
  (if (> _output_get (Variables|Default|GetSwitchTime))
    (Variables|Default|SetElapseTime 0.0)
    (if (Variables|Default|GetIsFire)
      (Variables|Default|SetIsFire false)
      (else
        (Variables|Default|SetIsFire true))))
  (return))