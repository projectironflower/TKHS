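; Monster actor whose mesh materials receive camera-to-player line proximity, apparently to fade it when it would block the view of the player.
; The construction script creates dynamic instances of one monster material on both mesh slots and sets fade start distance and power.
; Each tick measures the mesh origin's distance to the infinite line through the player's camera and capsule, feeding it to both materials.
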(event EventBeginPlay)

(event Collision|EventActorBeginOverlap
  (params (OtherActor :type Actor%20Object%20Reference)))

(event EventTick
  (params (DeltaSeconds :type Float%20%28single-precision%29))
  (bind _asplayer_bp (Utilities|Casting|CastToPlayer_BP (Game|Player|GetPlayerPawn 0)))
  (Rendering|Material|SetScalarParameterValue (Variables|Default|GetDynamicMaterial0) "DistanceToCameraVector" (Math|Vector|GetPointDistancetoLine (Transformation|GetWorldLocation (Variables|Debug|GetStaticMeshComponent)) (Transformation|GetWorldLocation (Variables|/Game/Content/Blueprint/Player/Player_BP.Player_BP_C|GetCamera _asplayer_bp)) (- (Transformation|GetWorldLocation (Variables|/Script/Engine.Character|GetCapsuleComponent _asplayer_bp)) (Transformation|GetWorldLocation (Variables|/Game/Content/Blueprint/Player/Player_BP.Player_BP_C|GetCamera _asplayer_bp)))) :!class /Script/Engine.MaterialInstanceDynamic)
  (Rendering|Material|SetScalarParameterValue (Variables|Default|GetDynamicMaterial1) "DistanceToCameraVector" (Math|Vector|GetPointDistancetoLine (Transformation|GetWorldLocation (Variables|Debug|GetStaticMeshComponent)) (Transformation|GetWorldLocation (Variables|/Game/Content/Blueprint/Player/Player_BP.Player_BP_C|GetCamera _asplayer_bp)) (- (Transformation|GetWorldLocation (Variables|/Script/Engine.Character|GetCapsuleComponent _asplayer_bp)) (Transformation|GetWorldLocation (Variables|/Game/Content/Blueprint/Player/Player_BP.Player_BP_C|GetCamera _asplayer_bp)))) :!class /Script/Engine.MaterialInstanceDynamic))

(fn ConstructionScript
  (Utilities|FlowControl|Sequence
    (:then_0
      (bind _returnvalue (Rendering|Material|CreateDynamicMaterialInstance (Variables|Debug|GetStaticMeshComponent) 0 "/Game/Content/Material/monster_tex_Mat2.monster_tex_Mat2" "None" :!class /Script/Engine.PrimitiveComponent))
      (bind _output_get (Variables|Default|SetDynamicMaterial0 _returnvalue))
      (Rendering|Material|SetScalarParameterValue _output_get "FadeStartDistance" (Variables|Default|GetFadeStartDistance) :!class /Script/Engine.MaterialInstanceDynamic)
      (Rendering|Material|SetScalarParameterValue (Variables|Default|GetDynamicMaterial0) "Power" (Variables|Default|GetPower) :!class /Script/Engine.MaterialInstanceDynamic))
    (:then_1
      (bind _returnvalue_2 (Rendering|Material|CreateDynamicMaterialInstance (Variables|Debug|GetStaticMeshComponent) 1 "/Game/Content/Material/monster_tex_Mat2.monster_tex_Mat2" "None" :!class /Script/Engine.PrimitiveComponent))
      (bind _output_get_2 (Variables|Default|SetDynamicMaterial1 _returnvalue_2))
      (Rendering|Material|SetScalarParameterValue _output_get_2 "FadeStartDistance" (Variables|Default|GetFadeStartDistance) :!class /Script/Engine.MaterialInstanceDynamic)
      (Rendering|Material|SetScalarParameterValue (Variables|Default|GetDynamicMaterial1) "Power" (Variables|Default|GetPower) :!class /Script/Engine.MaterialInstanceDynamic))))