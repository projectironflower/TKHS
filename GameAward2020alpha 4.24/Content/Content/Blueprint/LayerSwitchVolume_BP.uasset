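; Trigger volume that moves the player between back, front and base depth layers along world X.
; Tick polls whether the Player_BP box overlaps the volume's Box, then passes the player's vertical axis to SwitchLayer.
; Up or down input snaps X to the back or front offset when ToBack or ToFront allows it.
; With neither flag set, it snaps to base plus BaseXOffset regardless of input; BoxSize scales the root at construction.
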(event EventBeginPlay)

(event Collision|EventActorBeginOverlap
  (params (OtherActor :type Actor%20Object%20Reference)))

(event EventTick
  (params (DeltaSeconds :type Float%20%28single-precision%29))
  (bind _isoverlapping (CallFunction|IsOverlappingPlayer))
  (if _isoverlapping
    (CallFunction|SwitchLayer (Variables|/Game/Content/Blueprint/Player/Player_BP.Player_BP_C|GetAxisVertical (.AsPlayer%20BP (Utilities|Casting|CastToPlayer_BP (Game|Player|GetPlayerPawn 0)))))))

(fn ConstructionScript
  (Transformation|SetWorldScale3D (Variables|Default|GetDefaultSceneRoot) (/ (Variables|Default|GetBoxSize) 1e+02)))

(fn IsOverlappingPlayer
  (bind _returnvalue (Game|Player|GetPlayerPawn 0))
  (bind (_asplayer_bp _bsuccess) (Utilities|Casting|CastToPlayer_BP _returnvalue))
  (return (and _bsuccess (Class|PrimitiveComponent|IsOverlappingComponent (Variables|/Game/Content/Blueprint/Player/Player_BP.Player_BP_C|GetBox _asplayer_bp) (Variables|Default|GetBox)))))

(fn SwitchLayer
  (params (AxisVertical :type Float%20%28single-precision%29))
  (Utilities|FlowControl|Sequence
    (:then_0
      (if (and (> AxisVertical 0.0) (Variables|Default|GetToBack))
        (CallFunction|SwitchtoBack)
        (return)))
    (:then_1
      (if (and (< AxisVertical 0.0) (Variables|Default|GetToFront))
        (CallFunction|SwitchtoFront)
        (return)))
    (:then_2
      (if (Math|Boolean|NORBoolean (Variables|Default|GetToFront) (Variables|Default|GetToBack))
        (CallFunction|SwitchtoBase)
        (return)))))

(fn SwitchtoBack
  (bind _returnvalue (Game|Player|GetPlayerPawn 0))
  (bind _returnvalue_2 (Transformation|GetActorLocation _returnvalue))
  (bind (_x _y _z) (Math|Vector|BreakVector _returnvalue_2))
  (Transformation|SetActorLocation _returnvalue (Math|Vector|MakeVector (+ (.X (Math|Vector|BreakVector (Transformation|GetWorldLocation (Variables|Default|GetDefaultSceneRoot)))) 1.5e+02) _y _z) false false))

(fn SwitchtoFront
  (bind _returnvalue (Game|Player|GetPlayerPawn 0))
  (bind _returnvalue_2 (Transformation|GetActorLocation _returnvalue))
  (bind (_x _y _z) (Math|Vector|BreakVector _returnvalue_2))
  (Transformation|SetActorLocation _returnvalue (Math|Vector|MakeVector (+ (.X (Math|Vector|BreakVector (Transformation|GetWorldLocation (Variables|Default|GetDefaultSceneRoot)))) -5e+01) _y _z) false false))

(fn SwitchtoBase
  (bind _returnvalue (Game|Player|GetPlayerPawn 0))
  (bind _returnvalue_2 (Transformation|GetActorLocation _returnvalue))
  (bind (_x _y _z) (Math|Vector|BreakVector _returnvalue_2))
  (Transformation|SetActorLocation _returnvalue (Math|Vector|MakeVector (+ (.X (Math|Vector|BreakVector (Transformation|GetWorldLocation (Variables|Default|GetDefaultSceneRoot)))) 5e+01 (Variables|Default|GetBaseXOffset)) _y _z) false false))