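; Ice cube that the player pushes into place and that is shaved down by a shaved-ice machine.
; Tick nudges it along +Y while an overlapping Player_BP moves right; past SetLocationY, physics stops and it steps down toward FallLimit.
; Each ShaveIce call thins its Z scale, then hides it and disables collision; Respawn restores the scale cached at BeginPlay, visibility and collision.
; The Box overlap handler is a leftover with no effect.
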(event OnComponentBeginOverlap(Box)
  (params (OverlappedComponent :type Primitive%20Component%20Object%20Reference) (OtherActor :type Actor%20Object%20Reference) (OtherComp :type Primitive%20Component%20Object%20Reference) (OtherBodyIndex :type Integer) (bFromSweep :type Boolean) (SweepResult :type Hit%20Result%20Structure%20%28by%20ref%29))
  ;[1 1 1] 落下限界の設定の残骸
  (Variables|Default|SetNewVar_0 (Actor|ActorHasTag OtherActor "target"))
  (if true
    _))

(event Custom|Shave%20Ice
  (bind _ice_cube (Variables|Default|GetIce_Cube))
  (bind _ice_cube_2 (Variables|Default|GetIce_Cube))
  (bind _returnvalue (Transformation|GetWorldScale _ice_cube_2))
  ;[1 1 1] かき氷機で削られるとき
  (Physics|SetSimulatePhysics _ice_cube_2 false)
  (if (>= (.Z (Math|Vector|BreakVector _returnvalue)) 0.01)
    (Transformation|SetWorldScale3D _ice_cube_2 (- _returnvalue "0,0.000000,0.005000"))
    (else
      (Rendering|SetVisibility _ice_cube false false)
      (Collision|SetCollisionEnabled _ice_cube "NoCollision"))))

(event Custom|Respawn
  (bind _ice_cube (Variables|Default|GetIce_Cube))
  ;[1 1 1] サイズ復活
  (Transformation|SetWorldScale3D _ice_cube (Variables|Default|GetFullScale))
  (Rendering|SetVisibility _ice_cube true false)
  (Collision|SetCollisionEnabled _ice_cube "QueryAndPhysics"))

(event EventBeginPlay
  (Variables|Default|SetFullScale (Transformation|GetWorldScale (Variables|Default|GetIce_Cube))))

(event Collision|EventActorBeginOverlap
  (params (OtherActor :type Actor%20Object%20Reference)))

(event EventTick
  (params (DeltaSeconds :type Float%20%28single-precision%29))
  (bind _ice_cube (Variables|Default|GetIce_Cube))
  (bind _setlocationy (Variables|Default|GetSetLocationY))
  (bind _returnvalue (Transformation|GetWorldLocation _ice_cube))
  (bind (_x _y _z) (Math|Vector|BreakVector _returnvalue))
  ;[1 1 1] Tick
  (if (>= _y _setlocationy)
    (Physics|SetSimulatePhysics _ice_cube false)
    (if (>= _z (Variables|Default|GetFallLimit))
      (Transformation|SetWorldLocation (Variables|Default|GetIce_Cube) (Math|Vector|MakeVector _x _setlocationy (- _z (Variables|Default|GetFallSpeed))) false false))
    (else
      (CallFunction|MoveRight))))

(fn ConstructionScript)

(fn MoveRight
  (bind _ice_cube (Variables|Default|GetIce_Cube))
  (bind _returnvalue (Transformation|GetWorldLocation _ice_cube))
  (bind (_x _y _z) (Math|Vector|BreakVector _returnvalue))
  (for _array_element (Collision|GetOverlappingActors "/Game/Content/Blueprint/Player/Player_BP.Player_BP_C" :!class /Script/Engine.Actor)
    (bind _asplayer_bp (Utilities|Casting|CastToPlayer_BP _array_element))
    (if (> (Variables|/Game/Content/Blueprint/Player/Player_BP.Player_BP_C|GetIsRight _asplayer_bp) 0.0)
      (Transformation|SetWorldLocation _ice_cube (Math|Vector|MakeVector _x (+ _y (Variables|Default|GetMoveSpeed)) _z) false false))))