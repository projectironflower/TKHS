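; BeltConveyor_BP is a conveyor belt that pushes the player along the world Y axis while they are on it.
; Box overlap events with Player_BP set and clear IsOnPlayer.
; While set, Tick adds movement input to the player pawn, signed by ToRight and scaled by DeltaSeconds, MoveSpeed and Constant.
; The construction script sets the mesh material's Speed vector parameter to match the ToRight direction.
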(event OnComponentBeginOverlap(Box)
  (params (OverlappedComponent :type Primitive%20Component%20Object%20Reference) (OtherActor :type Actor%20Object%20Reference) (OtherComp :type Primitive%20Component%20Object%20Reference) (OtherBodyIndex :type Integer) (bFromSweep :type Boolean) (SweepResult :type Hit%20Result%20Structure%20%28by%20ref%29))
  (Utilities|Casting|CastToPlayer_BP OtherActor)
  (Variables|Default|SetIsOnPlayer true))

(event OnComponentEndOverlap(Box)
  (params (OverlappedComponent :type Primitive%20Component%20Object%20Reference) (OtherActor :type Actor%20Object%20Reference) (OtherComp :type Primitive%20Component%20Object%20Reference) (OtherBodyIndex :type Integer))
  (Utilities|Casting|CastToPlayer_BP OtherActor)
  (Variables|Default|SetIsOnPlayer false))

(event EventBeginPlay)

(event Collision|EventActorBeginOverlap
  (params (OtherActor :type Actor%20Object%20Reference)))

(event EventTick
  (params (DeltaSeconds :type Float%20%28single-precision%29))
  (bind _movespeed (Variables|Default|GetMoveSpeed))
  (bind _constant (Variables|Default|GetConstant))
  (bind _returnvalue (* DeltaSeconds _movespeed _constant))
  (if (Variables|Default|GetIsOnPlayer)
    (bind _asplayer_bp (Utilities|Casting|CastToPlayer_BP (Game|Player|GetPlayerPawn 0)))
    (if (Variables|Default|GetToRight)
      (Pawn|Input|AddMovementInput _asplayer_bp "0,1.000000, 0" _returnvalue false)
      (else
        (Pawn|Input|AddMovementInput _asplayer_bp "0,-1.000000, 0" _returnvalue false)))))

(fn ConstructionScript
  (bind _staticmesh (Variables|Default|GetStaticMesh))
  (if (Variables|Default|GetToRight)
    (Rendering|Material|SetVectorParameterValueonMaterials _staticmesh "Speed" "1.000000, 0, 0")
    (else
      (Rendering|Material|SetVectorParameterValueonMaterials _staticmesh "Speed" "-1.000000, 0, 0"))))