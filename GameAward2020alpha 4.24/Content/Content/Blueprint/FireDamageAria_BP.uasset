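; Fire hazard area actor that damages players standing inside its box trigger and shows a fire damage widget.
; Entering and leaving the box toggle the player's IsOnFire flag and notify the widget, which is created on BeginPlay and re-added to the viewport on exit.
; Tick applies damage every frame to overlapping players that are on fire and fires the ApplyFireDamage dispatcher.
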(event OnComponentBeginOverlap(Box)
  (params (OverlappedComponent :type Primitive%20Component%20Object%20Reference) (OtherActor :type Actor%20Object%20Reference) (OtherComp :type Primitive%20Component%20Object%20Reference) (OtherBodyIndex :type Integer) (bFromSweep :type Boolean) (SweepResult :type Hit%20Result%20Structure%20%28by%20ref%29))
  (bind (_asplayer_bp _bsuccess) (Utilities|Casting|CastToPlayer_BP OtherActor))
  (if _bsuccess
    (Variables|/Game/Content/Blueprint/Player/Player_BP.Player_BP_C|SetIsOnFire _asplayer_bp true)
    (Default|InDamageZone (Variables|Default|GetFireDamageUI))))

(event OnComponentEndOverlap(Box)
  (params (OverlappedComponent :type Primitive%20Component%20Object%20Reference) (OtherActor :type Actor%20Object%20Reference) (OtherComp :type Primitive%20Component%20Object%20Reference) (OtherBodyIndex :type Integer))
  (bind (_asplayer_bp _bsuccess) (Utilities|Casting|CastToPlayer_BP OtherActor))
  (bind _firedamageui (Variables|Default|GetFireDamageUI))
  (if _bsuccess
    (Variables|/Game/Content/Blueprint/Player/Player_BP.Player_BP_C|SetIsOnFire _asplayer_bp false)
    (Default|OutDamageZone _firedamageui)
    (Widget|RemovefromParent _firedamageui)
    (UserInterface|Viewport|AddtoViewport _firedamageui 0)))

(event EventBeginPlay
  (bind _returnvalue (UserInterface|CreateWidget "/Game/Content/UI/FireDamage.FireDamage_C"))
  (bind _output_get (Variables|Default|SetFireDamageUI _returnvalue))
  (UserInterface|Viewport|AddtoViewport _output_get 0))

(event Collision|EventActorBeginOverlap
  (params (OtherActor :type Actor%20Object%20Reference)))

(event EventTick
  (params (DeltaSeconds :type Float%20%28single-precision%29))
  (for _array_element (Collision|GetOverlappingActors (Variables|Default|GetBox) "/Game/Content/Blueprint/Player/Player_BP.Player_BP_C" :!class /Script/Engine.PrimitiveComponent)
    (bind _asplayer_bp (Utilities|Casting|CastToPlayer_BP _array_element))
    (if (Variables|/Game/Content/Blueprint/Player/Player_BP.Player_BP_C|GetIsOnFire _asplayer_bp)
      (Default|Damage _asplayer_bp (Variables|Default|GetFireDamage))
      (Default|CallApplyFireDamage))))

(fn ConstructionScript)