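; Trigger volume that turns the player's mesh to one of six configurable yaw angles while the player is inside it.
; Each Tick polls whether the player pawn's Box overlaps the volume's Box, then passes the player's vertical axis to SwitchDirection.
; SwitchDirection combines left/right facing with up, neutral or down input into a pattern index.
; GetYaw maps that index to a degree variable, adding 180 for left-facing patterns, and RotatePlayer applies it as world rotation.
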(event EventBeginPlay)

(event Collision|EventActorBeginOverlap
  (params (OtherActor :type Actor%20Object%20Reference)))

(event EventTick
  (params (DeltaSeconds :type Float%20%28single-precision%29))
  (bind _isoverlapping (CallFunction|IsOverlappingPlayer))
  (if _isoverlapping
    (CallFunction|SwitchDirection (Variables|/Game/Content/Blueprint/Player/Player_BP.Player_BP_C|GetAxisVertical (.AsPlayer%20BP (Utilities|Casting|CastToPlayer_BP (Game|Player|GetPlayerPawn 0)))))))

(fn ConstructionScript)

(fn IsOverlappingPlayer
  (bind _returnvalue (Game|Player|GetPlayerPawn 0))
  (bind (_asplayer_bp _bsuccess) (Utilities|Casting|CastToPlayer_BP _returnvalue))
  (return (and _bsuccess (Class|PrimitiveComponent|IsOverlappingComponent (Variables|/Game/Content/Blueprint/Player/Player_BP.Player_BP_C|GetBox _asplayer_bp) (Variables|Default|GetBox)))))

(fn SwitchDirection
  (params (AxisVertical :type Float%20%28single-precision%29))
  ;[1 1 1] 軸値の保存
  (LocalVariables|SetAxisValue AxisVertical)
  ;[1 1 1] プレイヤーの向き判別
  (bind _asplayer_bp (Utilities|Casting|CastToPlayer_BP (Game|Player|GetPlayerPawn 0)))
  (LocalVariables|SetPlayer _asplayer_bp)
  (if (> (Variables|/Game/Content/Blueprint/Player/Player_BP.Player_BP_C|GetIsRight _asplayer_bp) 0.0)
    ;[1 1 1] 軸値で場合分け
    (if (> (LocalVariables|GetAxisValue) 0.0)
      ;[1 1 1] プレイヤーを回転
      (CallFunction|RotatePlayer (LocalVariables|GetPlayer))
      (elif (< (LocalVariables|GetAxisValue) 0.0)
        (CallFunction|RotatePlayer (LocalVariables|GetPlayer) 2)
        (else
          (CallFunction|RotatePlayer (LocalVariables|GetPlayer) 1))))
    (return)
    (elif (< (Variables|/Game/Content/Blueprint/Player/Player_BP.Player_BP_C|GetIsRight _asplayer_bp) 0.0)
      (if (> (LocalVariables|GetAxisValue) 0.0)
        (CallFunction|RotatePlayer (LocalVariables|GetPlayer) 3)
        (elif (< (LocalVariables|GetAxisValue) 0.0)
          (CallFunction|RotatePlayer (LocalVariables|GetPlayer) 5)
          (else
            (CallFunction|RotatePlayer (LocalVariables|GetPlayer) 4))))
      (return))))

(fn RotatePlayer
  (params (Player :type Player%20BP%20Object%20Reference) (Puttern :type Integer))
  (bind _yaw (CallFunction|GetYaw Puttern))
  (Transformation|SetWorldRotation (Variables|/Script/Engine.Character|GetMesh Player) (Math|Rotator|MakeRotator 0.0 0.0 _yaw) false false))

(fn GetYaw
  (params (NewParam :type Integer))
  (return (Utilities|Array|Get(acopy) (Utilities|Array|MakeArray (Variables|Default|GetRightTopDegree) (Variables|Default|GetRightDegree) (Variables|Default|GetRightBotDegree) (+ (Variables|Default|GetLeftTopDegree) 1.8e+02) (+ (Variables|Default|GetLeftDegree) 1.8e+02) (+ (Variables|Default|GetLeftBotDegree) 1.8e+02)) NewParam)))