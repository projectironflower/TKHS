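; GirlSpawner_BP is a spawner that endlessly creates NPCGirl_BP characters at its own transform, starting on BeginPlay.
; Each new NPC receives movement and fall speeds, plus one coordinate from each of four referenced points (Y, X, Y, Z), apparently defining its route.
; SpawnCharacter re-calls itself after a SpawnRate delay, forming the spawn loop without Tick or a timer.
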(event Custom|SpawnCharacter
  (bind _returnvalue (Game|SpawnActorfromClass "/Game/Content/Blueprint/NPCSpawner/NPCGirl_BP.NPCGirl_BP_C" (Transformation|GetActorTransform) "Undefined" 0 0))
  (Variables|/Game/Content/Blueprint/NPCSpawner/NPCGirl_BP.NPCGirl_BP_C|Set1stY _returnvalue (.Y (Math|Vector|BreakVector (Transformation|GetActorLocation (Variables|Default|Get1stPoint)))))
  (Variables|/Game/Content/Blueprint/NPCSpawner/NPCGirl_BP.NPCGirl_BP_C|Set2ndX _returnvalue (.X (Math|Vector|BreakVector (Transformation|GetActorLocation (Variables|Default|Get2ndPoint)))))
  (Variables|/Game/Content/Blueprint/NPCSpawner/NPCGirl_BP.NPCGirl_BP_C|Set3rdY _returnvalue (.Y (Math|Vector|BreakVector (Transformation|GetActorLocation (Variables|Default|Get3rdPoint)))))
  (Variables|/Game/Content/Blueprint/NPCSpawner/NPCGirl_BP.NPCGirl_BP_C|Set4thZ _returnvalue (.Z (Math|Vector|BreakVector (Transformation|GetActorLocation (Variables|Default|Get4thPoint)))))
  (Variables|/Game/Content/Blueprint/NPCSpawner/NPCGirl_BP.NPCGirl_BP_C|SetMoveSpeed _returnvalue (Variables|Default|GetMoveSpeed))
  (Variables|/Game/Content/Blueprint/NPCSpawner/NPCGirl_BP.NPCGirl_BP_C|SetFallSpeed _returnvalue (Variables|Default|GetFallSpeed))
  (Utilities|FlowControl|Delay (Variables|Default|GetSpawnRate))
  (CallFunction|SpawnCharacter))

(event EventBeginPlay
  (CallFunction|SpawnCharacter))

(event Collision|EventActorBeginOverlap
  (params (OtherActor :type Actor%20Object%20Reference)))

(event EventTick
  (params (DeltaSeconds :type Float%20%28single-precision%29)))

(fn ConstructionScript)