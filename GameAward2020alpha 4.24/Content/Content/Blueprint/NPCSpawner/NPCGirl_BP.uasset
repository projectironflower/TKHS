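; NPC girl actor that moves along a fixed axis-aligned route, then drops and destroys itself.
; Tick switches on StateNumber to move it along +Y, -X and -Y at MoveSpeed, advancing as each coordinate threshold is crossed.
; The last state lowers it at FallSpeed until it reaches the Z limit and is destroyed.
; Movement sets the location directly without sweep, scaled by delta time to a 60 fps baseline.
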(event EventBeginPlay)

(event Collision|EventActorBeginOverlap
  (params (OtherActor :type Actor%20Object%20Reference)))

(event EventTick
  (params (DeltaSeconds :type Float%20%28single-precision%29))
  (bind _movespeed (Variables|Default|GetMoveSpeed))
  (bind _returnvalue (* _movespeed DeltaSeconds 6e+01))
  (switch int (Variables|Default|GetStateNumber)
    (:0
      (Transformation|SetActorLocation (+ (Transformation|GetActorLocation) (* "0,1.000000, 0" _returnvalue)) false false)
      (if (>= (.Y (Math|Vector|BreakVector (Transformation|GetActorLocation))) (Variables|Default|Get1stY))
        (Variables|Default|SetStateNumber 1)))
    (:1
      (Transformation|SetActorLocation (+ (Transformation|GetActorLocation) (* "-1.000000,0.000000, 0" _returnvalue)) false false)
      (if (<= (.X (Math|Vector|BreakVector (Transformation|GetActorLocation))) (Variables|Default|Get2ndX))
        (Variables|Default|SetStateNumber 2)))
    (:2
      (Transformation|SetActorLocation (+ (Transformation|GetActorLocation) (* "0.000000,-1.000000, 0" _returnvalue)) false false)
      (if (<= (.Y (Math|Vector|BreakVector (Transformation|GetActorLocation))) (Variables|Default|Get3rdY))
        (Variables|Default|SetStateNumber 3)))
    (:3
      (Transformation|SetActorLocation (+ (Transformation|GetActorLocation) (* "0.000000,0.000000,-1.000000" (* (Variables|Default|GetFallSpeed) DeltaSeconds 6e+01))) false false)
      (if (<= (.Z (Math|Vector|BreakVector (Transformation|GetActorLocation))) (Variables|Default|Get4thZ))
        (Actor|DestroyActor)))))

(fn ConstructionScript)