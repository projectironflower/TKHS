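; WaterBlock_BP is a water hazard block that deals 100 damage to the player on overlapping its DamageArea, until it is frozen.
; Freeze sets IsFreezed, swaps the visible Water component for Ice, and disables that damage through the flag check.
; It then recursively calls Freeze on WaterBlock_BP actors overlapping its ContactBox, so freezing spreads through connected blocks, with the flag preventing repeat visits.
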(event OnComponentBeginOverlap(DamageArea)
  (params (OverlappedComponent :type Primitive%20Component%20Object%20Reference) (OtherActor :type Actor%20Object%20Reference) (OtherComp :type Primitive%20Component%20Object%20Reference) (OtherBodyIndex :type Integer) (bFromSweep :type Boolean) (SweepResult :type Hit%20Result%20Structure%20%28by%20ref%29))
  (bind (_asplayer_bp _bsuccess) (Utilities|Casting|CastToPlayer_BP OtherActor))
  (if (not (Variables|Default|GetIsFreezed))
    (if _bsuccess
      (Default|Damage _asplayer_bp 1e+02))))

(event EventBeginPlay)

(event Collision|EventActorBeginOverlap
  (params (OtherActor :type Actor%20Object%20Reference)))

(event EventTick
  (params (DeltaSeconds :type Float%20%28single-precision%29)))

(fn ConstructionScript)

(fn Freeze
  (if (not (Variables|Default|GetIsFreezed))
    (Variables|Default|SetIsFreezed true)
    (Rendering|SetVisibility (Variables|Default|GetWater) false false)
    (Rendering|SetVisibility (Variables|Default|GetIce) true false)
    (for _array_element (Collision|GetOverlappingActors (Variables|Default|GetContactBox) "WaterBlock_BP_C" :!class /Script/Engine.PrimitiveComponent)
      (if (.bSuccess (Utilities|Casting|CastToWaterBlock_BP _array_element))
        (CallFunction|Freeze (.AsWater%20Block%20BP (Utilities|Casting|CastToWaterBlock_BP _array_element)))))))