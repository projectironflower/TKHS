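; Player character for a side-scrolling platformer along Y, whose life is its body volume.
; Moving, jumping, jetpack thrust, hard falls and freezing all feed Damage, which rescales the capsule, mass and jump velocity from remaining life, or triggers Death.
; Freezing turns overlapped water surfaces or fountains to ice via trigger references, with input locked meanwhile.
; Tick checks ice, movement cost and falls, while axis input switches between walking, ice sliding and block push/pull.
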(event Custom|GetJet
  ;[1 1 1] JetPack取得
  (Variables|フラグ|SetHaveJet true)
  (Rendering|SetVisibility (Variables|Default|GetJetPack) true false))

(event Custom|Damage
  (params (Damage :type Float%20%28single-precision%29))
  ;[1 1 1] ダメージ（体積減少全般）
  (if (not (Variables|フラグ|GetIsInvincible))
    (bind _output_get (Variables|パラメータ|SetLife (- (Variables|パラメータ|GetLife) Damage)))
    (if (> _output_get 0.0)
      (Utilities|CalcLifeRatio)
      (Transformation|SetWorldScale3D (Variables|Collision|GetCapsuleComponent) (Utilities|CalcNewScale))
      (Variables|/Script/Engine.CharacterMovementComponent|SetMass (Variables|Character|GetCharacterMovement) (* (Variables|一時変数|GetLifeRatio) (Variables|パラメータ初期値|GetMaxMass)))
      (Variables|/Script/Engine.CharacterMovementComponent|SetJumpZVelocity (Variables|Character|GetCharacterMovement) (Utilities|CalcJumpVelocity))
      (else
        (CallFunction|Death)))))

(event Custom|Death
  ;[1 1 1] Death
  (Utilities|FlowControl|DoOnce false
    (:Completed
      (Input|DisableInput (Game|GetPlayerController 0))
      (Pawn|Components|CharacterMovement|DisableMovement (Variables|Character|GetCharacterMovement))
      (Variables|フラグ|SetIsDead true)
      (bind _returnvalue (Effects|SpawnEmitteratLocation "/Game/Content/Particle/P_DeathSmoke.P_DeathSmoke" (Transformation|GetActorLocation)))
      (Variables|Default|SetDeathSmoke _returnvalue)
      (Audio|Components|Audio|Stop (Variables|Default|GetJetPack_Cue))
      (Audio|Components|Audio|Play (Variables|Default|GetBGM_Death_Cue) 0.0)
      (Default|CallStopBGM)
      (Utilities|FlowControl|Delay 0.8)
      (Rendering|SetActorHiddenInGame true)
      (Utilities|FlowControl|Delay 5.0)
      (Components|Activation|Deactivate (Variables|Default|GetDeathSmoke))
      (Default|CallPlayerDeath))))

(event Custom|Respawn
  ;[1 1 1] PlayerのRespawn時処理
  (Effects|SpawnEmitteratLocation "/Game/Content/Particle/P_DeathSmoke_Oneshot.P_DeathSmoke_Oneshot" (Transformation|GetActorLocation))
  (bind _scale (Timeline|タイムライン_0 Play)
    (:Update
      (Transformation|SetRelativeScale3D (Variables|Character|GetMesh) (* _scale 1.5)))))

(event Custom|OnClear
  (Input|DisableInput (Game|GetPlayerController 0))
  (Variables|軸値|SetAxisForword 0.0)
  (Variables|軸値|SetAxisVertical 0.0)
  (Variables|軸値|SetAxisGrab 0.0))

(event Custom|FreezeDamaging
  (bind _新規track_0 (Timeline|タイムライン_1 PlayFromStart)
    (:Update
      (CallFunction|Damage (* _新規track_0 (Utilities|Time|GetWorldDeltaSeconds) (Variables|パラメータ初期値|GetFreezeDamage))))))

(event EventBeginPlay
  (CallFunction|Damage 0.0)
  (bind _asmy_game_instance (Utilities|Casting|CastToMyGameInstance (Game|GetGameInstance)))
  (Variables|Default|SetGameInstance _asmy_game_instance))

(event Collision|EventActorBeginOverlap
  (params (OtherActor :type Actor%20Object%20Reference)))

(event EventTick
  (params (DeltaSeconds :type Float%20%28single-precision%29))
  ;[1 1 1] tick
  (CallFunction|CheckonIce)
  (CallFunction|MoveDamage DeltaSeconds)
  (Utilities|CalcFall))

(event EventOnJumped
  ;[1 1 1] ジャンプ関係
  (Effects|SpawnEmitteratLocation "/Game/Content/Particle/P_Jump.P_Jump" (Transformation|GetWorldLocation (Variables|Character|GetMesh)))
  (CallFunction|Damage (Variables|パラメータ初期値|GetJumpDamage))
  (Variables|フラグ|SetIsLanding false)
  (Audio|PlaySound2D "/Game/Content/Sound/SE/SE/Jump_Cue.Jump_Cue" 1.0 1.0 0.0 0 0))

(event EventOnLanded
  (params (Hit :type Hit%20Result%20Structure%20%28by%20ref%29))
  ;[1 1 1] ジャンプ関係
  (Variables|フラグ|SetIsLanding true)
  (Audio|PlaySound2D "/Game/Content/Sound/SE/SE/FootSteps1_Cue.FootSteps1_Cue" 1.0 1.0 0.0 0 0))

(event Input|ActionEvents|InputActionJump
  (params (Key :type Key%20Structure :default "None"))
  ;[1 1 1] ジャンプ関係
  (:Pressed
    (if (and (not (Variables|フラグ|GetHaveJet)) (<= (Variables|軸値|GetAxisGrab) 0.0))
      (Character|Jump))))

(event Input|ActionEvents|InputActionFreeze
  (params (Key :type Key%20Structure :default "None"))
  (bind _returnvalue (Game|GetPlayerController 0))
  (bind _returnvalue_2 (Game|GetPlayerController 0))
  ;[1 1 1] 凍らせる
  (:Pressed
    (if (Variables|フラグ|GetCanFreeze)
      (for _array_element (Collision|GetOverlappingActors (Variables|Collision|GetCapsuleComponent) "/Game/Content/Blueprint/FreezeTrigger_BP.FreezeTrigger_BP_C" :!class /Script/Engine.PrimitiveComponent)
        (if (.bSuccess (Utilities|Casting|CastToFreezeTrigger_BP _array_element))
          (Utilities|FlowControl|Sequence
            (:then_0
              (bind _aswater_surface_bp (Utilities|Casting|CastToWaterSurface_BP (Variables|/Game/Content/Blueprint/FreezeTrigger_BP.FreezeTrigger_BP_C|GetReferencedWater (.AsFreeze%20Trigger%20BP (Utilities|Casting|CastToFreezeTrigger_BP _array_element)))))
              (if (not (Variables|/Game/Content/Blueprint/WaterSurface_BP.WaterSurface_BP_C|GetIsFreezed _aswater_surface_bp))
                (CallFunction|FreezeDamaging)
                (Effects|SpawnEmitteratLocation "/Game/Content/Particle/cold.cold" (+ (.Location (Math|Transform|BreakTransform (Transformation|GetActorTransform))) (Math|Vector|MakeVector 0.0 (* (Variables|フラグ|GetIsRight) 5e+01) 0.0)) "0, 0,120.000000" "1.200000,1.200000,1.200000")
                (Input|DisableInput _returnvalue_2)
                (Audio|Components|Audio|FadeIn (Variables|Default|GetBlizzard_Breath_Cue) 0.5 1.0 0.0 "Linear" :!class /Script/Engine.AudioComponent)
                (Variables|フラグ|SetIsFreezing true)
                (Utilities|FlowControl|Delay 0.8)
                (Audio|Components|Audio|FadeOut (Variables|Default|GetBlizzard_Breath_Cue) 1.0 0.0 "SCurve" :!class /Script/Engine.AudioComponent)
                (Audio|Components|Audio|FadeIn (Variables|Default|GetFreeze2_Cue) 1.0 1.0 0.0 "SCurve" :!class /Script/Engine.AudioComponent)
                (Default|Freeze _aswater_surface_bp true)
                (Utilities|FlowControl|Delay 0.2)
                (Input|EnableInput _returnvalue_2)
                (Variables|フラグ|SetIsFreezing false)
                (Default|CallFreeze)))
            (:then_1
              (bind _asfountain_bp (Utilities|Casting|CastToFountain_BP (Variables|/Game/Content/Blueprint/FreezeTrigger_BP.FreezeTrigger_BP_C|GetReferencedWater (.AsFreeze%20Trigger%20BP (Utilities|Casting|CastToFreezeTrigger_BP _array_element)))))
              (if (not (Variables|/Game/Content/Blueprint/Fountain_BP.Fountain_BP_C|GetIsFreezed _asfountain_bp))
                (CallFunction|FreezeDamaging)
                (Effects|SpawnEmitteratLocation "/Game/Content/Particle/cold.cold" (+ (.Location (Math|Transform|BreakTransform (Transformation|GetActorTransform))) (Math|Vector|MakeVector 0.0 (* (Variables|フラグ|GetIsRight) 5e+01) 0.0)) "0, 0,120.000000" "1.200000,1.200000,1.200000")
                (Input|DisableInput _returnvalue)
                (Audio|Components|Audio|FadeIn (Variables|Default|GetBlizzard_Breath_Cue) 0.5 1.0 0.0 "Linear" :!class /Script/Engine.AudioComponent)
                (Variables|フラグ|SetIsFreezing true)
                (Utilities|FlowControl|Delay 0.8)
                (Audio|Components|Audio|FadeOut (Variables|Default|GetBlizzard_Breath_Cue) 1.0 0.0 "SCurve" :!class /Script/Engine.AudioComponent)
                (Audio|Components|Audio|FadeIn (Variables|Default|GetFreeze2_Cue) 1.0 1.0 0.0 "SCurve" :!class /Script/Engine.AudioComponent)
                (Default|Freeze _asfountain_bp true)
                (Utilities|FlowControl|Delay 0.2)
                (Input|EnableInput _returnvalue)
                (Variables|フラグ|SetIsFreezing false)
                (Default|CallFreeze)))))))))

(event Input|ActionEvents|InputActionPauseButton
  (params (Key :type Key%20Structure :default "None"))
  (:Pressed
    (bind _returnvalue (Game|GetCurrentLevelName true))
    (if (not (Utilities|Enum|Equal(Enum) _returnvalue "StageSelect"))
      (Default|CallPause (Variables|Default|GetGameInstance)))))

(event Input|AxisEvents|InputAxisMoveForward
  (params (AxisValue :type Float%20%28single-precision%29))
  ;[1 1 1] 移動及び向き変更
  (Variables|軸値|SetAxisForword AxisValue)
  (if (not (Variables|フラグ|GetIsOnIce))
    (if (not (Variables|フラグ|GetIsGrabbing))
      (CallFunction|MoveForword (Math|Float|Absolute(Float) (Variables|軸値|GetAxisForword)))
      (CallFunction|Turn)
      (if (> (Variables|軸値|GetAxisForword) 0.0)
        (Variables|フラグ|SetIsRight 1.0)
        (elif (< (Variables|軸値|GetAxisForword) 0.0)
          (Variables|フラグ|SetIsRight -1.0)))
      (else
        (CallFunction|MoveCarry)))
    (else
      (CallFunction|MoveonIce))))

(event Input|AxisEvents|InputAxisJet
  (params (AxisValue :type Float%20%28single-precision%29))
  ;[1 1 1] ジェットパック
  (if (Variables|フラグ|GetHaveJet)
    (Utilities|FlowControl|Sequence
      (:then_0
        (if (> AxisValue 0.0)
          (Physics|AddForce (Variables|Character|GetCharacterMovement) (Math|Vector|MakeVector 0.0 0.0 (* (Variables|/Script/Engine.CharacterMovementComponent|GetMass (Variables|Character|GetCharacterMovement)) 2e+03)))
          (CallFunction|Damage (* (Variables|パラメータ初期値|GetJetDamage) (Utilities|Time|GetWorldDeltaSeconds) 6e+01))
          (Utilities|FlowControl|DoOnce false :!label _label
            (:Completed
              (Audio|Components|Audio|Play (Variables|Default|GetJetPack_Cue) 0.0)))
          (else
            (Audio|Components|Audio|Stop (Variables|Default|GetJetPack_Cue))
            (goto _label Reset))))
      (:then_1
        (if (< AxisValue 0.01)
          (Utilities|FlowControl|DoOnce false :!label _label_2
            (:Completed
              (Components|Activation|SetActive (Variables|Default|GetJetParticle) false false)))
          (else
            (goto _label_2 Reset))))
      (:then_2
        (if (> AxisValue 0.0)
          (Utilities|FlowControl|DoOnce false :!label _label_3
            (:Completed
              (Components|Activation|SetActive (Variables|Default|GetJetParticle) true false)))
          (else
            (goto _label_3 Reset)))))))

(event Input|AxisEvents|InputAxisMoveVertical
  (params (AxisValue :type Float%20%28single-precision%29))
  ;[1 1 1] 垂直方向軸値
  (Variables|軸値|SetAxisVertical AxisValue))

(event Input|AxisEvents|InputAxisGrab
  (params (AxisValue :type Float%20%28single-precision%29))
  ;[1 1 1] Grab
  (Variables|軸値|SetAxisGrab AxisValue))

(fn ConstructionScript)

(fn GetSpeed
  (bind _returnvalue (Transformation|GetVelocity))
  (bind (_x _y) (Math|Vector|BreakVector _returnvalue))
  (return (Math|Vector|VectorLength (Math|Vector|MakeVector _x _y 0.0))))

(fn CheckonIce
  (bind _array_element (Utilities|Array|ForEachLoopwithBreak (Collision|GetOverlappingActors (Variables|Collision|GetCapsuleComponent) "/Game/Content/Blueprint/WaterSurface_BP.WaterSurface_BP_C" :!class /Script/Engine.PrimitiveComponent) :!label _label)
    (:LoopBody
      (if (and (Variables|/Game/Content/Blueprint/WaterSurface_BP.WaterSurface_BP_C|GetIsFreezed (.AsWater%20Surface%20BP (Utilities|Casting|CastToWaterSurface_BP _array_element))) (.bSuccess (Utilities|Casting|CastToWaterSurface_BP _array_element)))
        (if (.bSuccess (Utilities|Casting|CastToPlayer_BP (Utilities|Array|Get(acopy) (Collision|GetOverlappingActors (Variables|/Game/Content/Blueprint/WaterSurface_BP.WaterSurface_BP_C|GetBox (.AsWater%20Surface%20BP (Utilities|Casting|CastToWaterSurface_BP _array_element))) "Player_BP_C" :!class /Script/Engine.PrimitiveComponent))))
          (Math|Integer|IncrementInt (Variables|一時変数|GetNumIce)
            (:%20%20
              (goto _label Break))))))
    (:Completed
      (if (> (Variables|一時変数|GetNumIce) 0)
        (Variables|フラグ|SetIsOnIce true)
        (else
          (Variables|フラグ|SetIsOnIce false)))
      (Variables|一時変数|SetNumIce 0))))

(fn MoveDamage
  (params (A :type Float%20%28single-precision%29))
  (bind _movedamagepartical (Variables|Default|GetMoveDamagePartical))
  (if (> (Math|Float|Absolute(Float) (Variables|軸値|GetAxisForword)) 0.01)
    (if (Variables|フラグ|GetIsOnIce)
      (Components|Activation|Activate _movedamagepartical false)
      (CallFunction|Damage (* A (Variables|パラメータ初期値|GetDamageMoveIce)))
      (else
        (Components|Activation|Activate _movedamagepartical false)
        (CallFunction|Damage (* A (Variables|パラメータ初期値|GetDamageMove)))))
    (else
      (Components|Activation|Deactivate (Variables|Default|GetMoveDamagePartical)))))

(fn MoveonIce
  (Pawn|Input|AddMovementInput "0,1.000000, 0" (.Y (Math|Vector|BreakVector (Variables|/Script/Engine.MovementComponent|GetVelocity (Variables|Character|GetCharacterMovement)))) true)
  (return))

(fn MoveForword
  (params (ScaleValue :type Float%20%28single-precision%29))
  (Pawn|Input|AddMovementInput (Math|Vector|GetRightVector (Variables|Character|GetMesh)) ScaleValue false))

(fn Turn
  (bind _mesh (Variables|Character|GetMesh))
  (bind _returnvalue (Transformation|GetWorldRotation _mesh))
  (bind (_roll _pitch _yaw) (Math|Rotator|BreakRotator _returnvalue))
  (if (or (Variables|フラグ|GetIsLanding) (Variables|フラグ|GetHaveJet))
    (if (< (* (Variables|軸値|GetAxisForword) (.Y (Math|Vector|BreakVector (Math|Vector|GetRightVector (Variables|Character|GetMesh))))) 0.0)
      (Transformation|SetWorldRotation _mesh (Math|Rotator|MakeRotator _roll _pitch (+ _yaw 1.8e+02)) false false))))

(fn MoveCarry
  (bind _returnvalue (Transformation|GetActorLocation))
  (bind _mesh (Variables|Character|GetMesh))
  (bind _axisforword (Variables|軸値|GetAxisForword))
  (bind _grabbingobject (Variables|一時変数|GetGrabbingObject))
  (bind _grabbingobjectdistance (Variables|一時変数|GetGrabbingObjectDistance))
  (bind _returnvalue_2 (Transformation|GetActorLocation _grabbingobject))
  (bind _returnvalue_3 (Math|Vector|GetRightVector _mesh))
  (bind _returnvalue_4 (+ _returnvalue _grabbingobjectdistance))
  (bind (_x _y) (Math|Vector|BreakVector _returnvalue_4))
  (bind (_x_2 _y_2 _z) (Math|Vector|BreakVector _returnvalue_2))
  (bind _y_3 (Math|Vector|BreakVector _returnvalue_3))
  (bind _returnvalue_5 (* _axisforword _y_3))
  (Pawn|Input|AddMovementInput (Math|Vector|GetRightVector (Variables|Character|GetMesh)) (* (Variables|パラメータ|GetCarrySpeed) (Variables|軸値|GetAxisForword) 1.0) false)
  (bind _asmovable_block_bp (Utilities|Casting|CastToMovableBlock_BP _grabbingobject))
  (Utilities|FlowControl|Sequence
    (:then_0
      (if (> _returnvalue_5 0.0)
        (Variables|フラグ|SetIsPussing true)
        (Variables|フラグ|SetIsPulling false)
        (elif (< _returnvalue_5 0.0)
          (Variables|フラグ|SetIsPussing false)
          (Variables|フラグ|SetIsPulling true)
          (elif true
            (Variables|フラグ|SetIsPussing false)
            (Variables|フラグ|SetIsPulling false)))))
    (:then_1
      (if (Math|Boolean|NANDBoolean (>= (Variables|軸値|GetAxisForword) 0.0) (> _y_2 (Variables|/Game/Content/Blueprint/MovableBlock_BP.MovableBlock_BP_C|GetLimitY _asmovable_block_bp)))
        (Transformation|SetActorLocation _grabbingobject (Math|Vector|MakeVector _x _y _z) false false)))))