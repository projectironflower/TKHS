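; Movable block that the player can grab and carry while standing inside its Box trigger.
; While overlapped, Tick checks grab input and CheckCanGrab, then a DoOnce hands the player the block, carry speed and offset; release or exit clears grabbing.
; Move shifts the block without sweep along the player mesh's right vector by forward input, but is not called here.
; CheckCanGrab's facing test is left unconnected.
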(event OnComponentBeginOverlap(Box)
  (params (OverlappedComponent :type Primitive%20Component%20Object%20Reference) (OtherActor :type Actor%20Object%20Reference) (OtherComp :type Primitive%20Component%20Object%20Reference) (OtherBodyIndex :type Integer) (bFromSweep :type Boolean) (SweepResult :type Hit%20Result%20Structure%20%28by%20ref%29))
  (Utilities|Casting|CastToPlayer_BP OtherActor)
  (Variables|Default|SetOnPlayer true))

(event OnComponentEndOverlap(Box)
  (params (OverlappedComponent :type Primitive%20Component%20Object%20Reference) (OtherActor :type Actor%20Object%20Reference) (OtherComp :type Primitive%20Component%20Object%20Reference) (OtherBodyIndex :type Integer))
  (bind _asplayer_bp (Utilities|Casting|CastToPlayer_BP OtherActor))
  (Variables|Default|SetOnPlayer false)
  (Variables|/Game/Content/Blueprint/Player/Player_BP.Player_BP_C|SetIsGrabbing _asplayer_bp false))

(event EventBeginPlay)

(event Collision|EventActorBeginOverlap
  (params (OtherActor :type Actor%20Object%20Reference)))

(event EventTick
  (params (DeltaSeconds :type Float%20%28single-precision%29))
  (if (Variables|Default|GetOnPlayer)
    (bind _asplayer_bp (Utilities|Casting|CastToPlayer_BP (Game|Player|GetPlayerPawn 0)))
    (if (and (> (Variables|/Game/Content/Blueprint/Player/Player_BP.Player_BP_C|GetAxisGrab _asplayer_bp) 0.0) (Utilities|CheckCanGrab))
      (Utilities|FlowControl|DoOnce false :!label _label
        (:Completed
          (Variables|/Game/Content/Blueprint/Player/Player_BP.Player_BP_C|SetIsGrabbing _asplayer_bp true)
          (Variables|/Game/Content/Blueprint/Player/Player_BP.Player_BP_C|SetGrabbingObject _asplayer_bp self)
          (Variables|/Game/Content/Blueprint/Player/Player_BP.Player_BP_C|SetCarrySpeed _asplayer_bp (Variables|Default|GetMoveSpeed))
          (Variables|/Game/Content/Blueprint/Player/Player_BP.Player_BP_C|SetGrabbingObjectDistance _asplayer_bp (- (Transformation|GetActorLocation) (Transformation|GetActorLocation _asplayer_bp)))))
      (else
        (Variables|/Game/Content/Blueprint/Player/Player_BP.Player_BP_C|SetIsGrabbing _asplayer_bp false)
        (goto _label Reset)))))

(fn ConstructionScript)

(fn Move
  (params (DeltaSecond :type Float%20%28single-precision%29) (Player :type Player%20BP%20Object%20Reference))
  (Transformation|SetActorLocation (+ (* (Math|Vector|GetRightVector (Variables|/Script/Engine.Character|GetMesh Player)) (* (Variables|Default|GetMoveSpeed) (* DeltaSecond 6e+01) (Variables|/Game/Content/Blueprint/Player/Player_BP.Player_BP_C|GetAxisForword Player))) (Transformation|GetActorLocation)) false false))