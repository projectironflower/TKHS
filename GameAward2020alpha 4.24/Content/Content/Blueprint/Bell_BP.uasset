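; Bell actor that reacts when the player enters its trigger box, acting as a switch that starts a sequence.
; On overlap it casts to Player_BP and requires the player's CharacterMovement mass to be above zero.
; It then nudges the bell mesh down with a sweep, plays a 2D bell sound and calls BeginSequence.
; Nothing resets the mesh or guards against repeats, so each qualifying overlap lowers it further.
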(event OnComponentBeginOverlap(Box)
  (params (OverlappedComponent :type Primitive%20Component%20Object%20Reference) (OtherActor :type Actor%20Object%20Reference) (OtherComp :type Primitive%20Component%20Object%20Reference) (OtherBodyIndex :type Integer) (bFromSweep :type Boolean) (SweepResult :type Hit%20Result%20Structure%20%28by%20ref%29))
  (bind (_asplayer_bp _bsuccess) (Utilities|Casting|CastToPlayer_BP OtherActor))
  (bind _bell_object001 (Variables|Default|Getbell_Object001))
  (if _bsuccess
    (if (> (Variables|/Script/Engine.CharacterMovementComponent|GetMass (Variables|/Script/Engine.Character|GetCharacterMovement _asplayer_bp)) 0.0)
      (Transformation|SetWorldLocation _bell_object001 (- (Transformation|GetWorldLocation _bell_object001) "0,0.000000,5.000000") true false)
      (Audio|PlaySound2D "/Game/Content/Sound/SE/SE_Bell.SE_Bell" 1.0 1.0 0.0 0 0)
      (Default|CallBeginSequence))))

(event EventBeginPlay)

(event Collision|EventActorBeginOverlap
  (params (OtherActor :type Actor%20Object%20Reference)))

(event EventTick
  (params (DeltaSeconds :type Float%20%28single-precision%29)))

(fn ConstructionScript)