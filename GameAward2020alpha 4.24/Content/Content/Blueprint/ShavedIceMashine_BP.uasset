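; Shaved-ice machine that spins and lowers a press while telling its linked IceCube_BP to shave, with a looping state cycle run on Tick.
; Shave alternates a press stroke, a reverse lift and a delay, toggling the shave sound and scaling steps by frame time.
; Player overlap with the Box freezes only the downward stroke's motion.
; The ice cube's move event halts the machine until Reset clears it.
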(event OnComponentBeginOverlap(Box)
  (params (OverlappedComponent :type Primitive%20Component%20Object%20Reference) (OtherActor :type Actor%20Object%20Reference) (OtherComp :type Primitive%20Component%20Object%20Reference) (OtherBodyIndex :type Integer) (bFromSweep :type Boolean) (SweepResult :type Hit%20Result%20Structure%20%28by%20ref%29))
  (if (.bSuccess (Utilities|Casting|CastToPlayer_BP OtherActor))
    (Variables|Default|SetIsPlayerOverlap true)))

(event OnComponentEndOverlap(Box)
  (params (OverlappedComponent :type Primitive%20Component%20Object%20Reference) (OtherActor :type Actor%20Object%20Reference) (OtherComp :type Primitive%20Component%20Object%20Reference) (OtherBodyIndex :type Integer))
  (if (.bSuccess (Utilities|Casting|CastToPlayer_BP OtherActor))
    (Variables|Default|SetIsPlayerOverlap false)))

(event Custom|Shave
  (bind _spiningobj (Variables|Default|GetSpiningObj))
  (bind _pressspeed (Variables|Default|GetPressSpeed))
  (bind _spinspeed (Variables|Default|GetSpinSpeed))
  (bind _press (Variables|Default|GetPress))
  (bind _returnvalue (Transformation|GetWorldRotation _spiningobj))
  (bind _returnvalue_2 (Transformation|GetWorldLocation _press))
  (bind _output (Utilities|ApplyValueatFPS _spinspeed))
  (bind _output_2 (Utilities|ApplyValueatFPS _pressspeed))
  ;[1 1 1] 氷を削るときのかき氷機の動き
  (if (Variables|Default|GetIsShave)
    (if (not (Variables|Default|GetIsPlayerOverlap))
      (Transformation|SetWorldRotation _spiningobj (Math|Rotator|MakeRotator (.roll _returnvalue) (.pitch _returnvalue) (+ (.yaw _returnvalue) _output)) false false)
      (Transformation|SetWorldLocation _press (Math|Vector|MakeVector (.x _returnvalue_2) (.y _returnvalue_2) (- (.z _returnvalue_2) _output_2)) false false)
      (Variables|Default|SetElapseTime (+ (Variables|Default|GetElapseTime) (Utilities|ApplyValueatFPS (Variables|Default|GetPressSpeed))))
      (if (> (+ (Variables|Default|GetElapseTime) (Utilities|ApplyValueatFPS (Variables|Default|GetPressSpeed))) 185.0)
        (Variables|Default|SetIsShave false)
        (Variables|Default|SetElapseTime 0.0)
        (Variables|Default|SetIsRespawnIce false)
        (Class|AudioComponent|SetPaused (Variables|Default|GetShaveSE) true)
        (Variables|Default|SetIsPlayerOverlap true)))
    (elif (< (Variables|Default|GetElapseTime) 185.0)
      (Transformation|SetWorldRotation _spiningobj (Math|Rotator|MakeRotator (.roll _returnvalue) (.pitch _returnvalue) (- (.yaw _returnvalue) _output)) false false)
      (Transformation|SetWorldLocation _press (Math|Vector|MakeVector (.x _returnvalue_2) (.y _returnvalue_2) (+ (.z _returnvalue_2) _output_2)) false false)
      (Variables|Default|SetElapseTime (+ (Variables|Default|GetElapseTime) (Utilities|ApplyValueatFPS (Variables|Default|GetPressSpeed))))
      (else
        (bind _output_get (Variables|Default|SetElapleDelayTime (+ (Variables|Default|GetElapleDelayTime) (Utilities|ApplyValueatFPS 1.0))))
        (if (> _output_get (Variables|Default|GetDelayTime))
          (Variables|Default|SetIsShave true)
          (Variables|Default|SetElapseTime 0.0)
          (Variables|Default|SetElapleDelayTime 0.0)
          (Class|AudioComponent|SetPaused (Variables|Default|GetShaveSE) false))))))

(event Custom|IceCubeMove
  (Variables|Default|SetIsMoveIceCube true))

(event Custom|Reset
  (Variables|Default|SetIsMoveIceCube false)
  (Variables|Default|SetIsPlayerOverlap false)
  (Variables|Default|SetIsShave false)
  (Variables|Default|SetIsRespawnIce false)
  (Variables|Default|SetElapseTime 185.0))

(event EventBeginPlay
  (bind _asice_cube_bp (Utilities|Casting|CastToIceCube_BP (Variables|Default|GetSetObject)))
  (bind _output_get (Variables|Default|SetIceCube _asice_cube_bp))
  (EventDispatchers|BindEventtoMoveRightObject _output_get (delegate Custom|IceCubeMove))
  (bind _returnvalue (Audio|CreateSound2D "/Game/Content/Sound/SE/SE_Shave.SE_Shave" 1.0 1.0 0.0 0 false false))
  (bind _returnvalue_2 (Audio|SpawnSoundAttached "/Game/Content/Sound/SE/SE_Shave.SE_Shave" _returnvalue "None" (Transformation|GetWorldLocation (Variables|Default|GetStaticMesh)) "0, 0, 0" "KeepRelativeOffset" false 1.0 1.0 0.0 "/Game/Content/Sound/SoundAttenuation.SoundAttenuation" 0 false))
  (bind _output_get_2 (Variables|Default|SetShaveSE _returnvalue_2))
  (Class|AudioComponent|SetPaused _output_get_2 true))

(event Collision|EventActorBeginOverlap
  (params (OtherActor :type Actor%20Object%20Reference)))

(event EventTick
  (params (DeltaSeconds :type Float%20%28single-precision%29))
  (if (Variables|Default|GetIsMoveIceCube)
    (Class|AudioComponent|SetPaused (Variables|Default|GetShaveSE) true)
    (else
      (CallFunction|Shave)
      (if (Variables|Default|GetIsShave)
        (Default|ShaveIce (Variables|Default|GetIceCube) (Utilities|Time|GetWorldDeltaSeconds))))))

(fn ConstructionScript)