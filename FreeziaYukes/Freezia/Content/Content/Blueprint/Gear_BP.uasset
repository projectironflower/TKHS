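; Gear actor that spins continuously around its local roll axis and plays a sound at its location on BeginPlay.
; Tick adds a local rotation each frame from DeltaSeconds and RotateSpeed, with the Reverse flag negating the direction.
; RotateSpeed passes through ApplyValueAtFPS, whose graph holds an apparently unconnected 60 FPS delta-time scaling expression.
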(event EventBeginPlay
  (Audio|PlaySoundatLocation 0 (Transformation|GetActorLocation) "0, 0, 0" 0.005 1.0 0.0 0 0 0))

(event Collision|EventActorBeginOverlap
  (params (OtherActor :type Actor%20Object%20Reference)))

(event EventTick
  (params (DeltaSeconds :type Float%20%28single-precision%29))
  (if (Variables|Default|GetReverse)
    (Transformation|AddActorLocalRotation (Math|Rotator|MakeRotator (* (* DeltaSeconds (Utilities|ApplyValueatFPS (Variables|Default|GetRotateSpeed))) -1.0) 0.0 0.0) false false)
    (else
      (Transformation|AddActorLocalRotation (Math|Rotator|MakeRotator (* DeltaSeconds (Utilities|ApplyValueatFPS (Variables|Default|GetRotateSpeed))) 0.0 0.0) false false))))

(fn ConstructionScript)