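; A water surface actor that switches its plane's material between water and ice as the water freezes or melts.
; On BeginPlay it binds Freeze and Melt handlers to the WaterBlock's OnFreezed and OnMelted events, each setting the matching material on the Plane.
; The construction script applies the same choice from the IsFreezed flag, so the initial state shows in the editor.
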(event Custom|Freeze
  (Rendering|Material|SetMaterial (Variables|Default|GetPlane) 0 "/Game/Content/Blueprint/Material/T_IceShards_E_Mat.T_IceShards_E_Mat"))

(event Custom|Melt
  (Rendering|Material|SetMaterial (Variables|Default|GetPlane) 0 "/Game/Content/Blueprint/Material/M_Water1.M_Water1"))

(event EventBeginPlay
  (bind _waterblock (Variables|Default|GetWaterBlock))
  (EventDispatchers|BindEventtoOnFreezed _waterblock (delegate Custom|Freeze))
  (EventDispatchers|BindEventtoOnMelted _waterblock (delegate Custom|Melt)))

(event Collision|EventActorBeginOverlap
  (params (OtherActor :type Actor%20Object%20Reference)))

(event EventTick
  (params (DeltaSeconds :type Float%20%28single-precision%29)))

(fn ConstructionScript
  (bind _plane (Variables|Default|GetPlane))
  (if (Variables|Default|GetIsFreezed)
    (Rendering|Material|SetMaterial _plane 0 "/Game/Content/Blueprint/Material/T_IceShards_E_Mat.T_IceShards_E_Mat")
    (else
      (Rendering|Material|SetMaterial _plane 0 "/Game/Content/Blueprint/Material/M_Water1.M_Water1"))))