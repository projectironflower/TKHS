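; Spawner actor that places a Memory_Piece at its own transform and replaces it on respawn.
; On BeginPlay it spawns the piece, binds its destruction to set an IsRespawn flag, and listens to the GameMode_BP OnRespawn dispatcher.
; On respawn, a set flag spawns a new piece and calls OnRespawn.
; The flag is never cleared, and replacement pieces get no destruction binding.
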(event Custom|SetRespawn
  (params (DestroyedActor :type Actor%20Object%20Reference))
  (Variables|Default|SetIsRespawn true))

(event Custom|Respawn
  (if (Variables|Default|GetIsRespawn)
    (Game|SpawnActorfromClass "/Game/Content/Blueprint/Memory_Piece.Memory_Piece_C" (Transformation|GetActorTransform) "Undefined" 0 0)
    (Default|CallOnRespawn)))

(event EventBeginPlay
  (bind _returnvalue (Game|SpawnActorfromClass "/Game/Content/Blueprint/Memory_Piece.Memory_Piece_C" (Transformation|GetActorTransform) "Undefined" 0 0))
  (Game|BindEventtoOnDestroyed _returnvalue (delegate Custom|SetRespawn))
  (bind _asgame_mode_bp (Utilities|Casting|CastToGameMode_BP (Game|GetGameMode)))
  (EventDispatchers|BindEventtoOnRespawn _asgame_mode_bp (delegate Custom|Respawn)))

(event Collision|EventActorBeginOverlap
  (params (OtherActor :type Actor%20Object%20Reference)))

(event EventTick
  (params (DeltaSeconds :type Float%20%28single-precision%29)))

(fn ConstructionScript)