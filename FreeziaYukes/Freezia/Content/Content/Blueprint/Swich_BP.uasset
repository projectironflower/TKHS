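; A floor-style switch that sinks when the player enters its trigger box.
; Tick lowers the switch mesh until it is 25 units below its start height, then calls SwitchOnObject, which is empty here.
; If pressure-sensitive, it rises back to its start height once the player leaves.
; Each movement step passes through the ApplyValueAtFPS helper, named for frame-rate compensation.
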(event OnComponentBeginOverlap(Box)
  (params (OverlappedComponent :type Primitive%20Component%20Object%20Reference) (OtherActor :type Actor%20Object%20Reference) (OtherComp :type Primitive%20Component%20Object%20Reference) (OtherBodyIndex :type Integer) (bFromSweep :type Boolean) (SweepResult :type Hit%20Result%20Structure%20%28by%20ref%29))
  (Utilities|Casting|CastToPlayer_BP OtherActor)
  (Variables|Default|SetIsSwitchOnObject true))

(event OnComponentEndOverlap(Box)
  (params (OverlappedComponent :type Primitive%20Component%20Object%20Reference) (OtherActor :type Actor%20Object%20Reference) (OtherComp :type Primitive%20Component%20Object%20Reference) (OtherBodyIndex :type Integer))
  (Utilities|Casting|CastToPlayer_BP OtherActor)
  (Variables|Default|SetIsOnActor false))

(event Custom|SwitchOnObject)

(event EventBeginPlay
  (Variables|Default|SetStartVector (Transformation|GetWorldLocation (Variables|Default|GetSwitch))))

(event Collision|EventActorBeginOverlap
  (params (OtherActor :type Actor%20Object%20Reference)))

(event EventTick
  (params (DeltaSeconds :type Float%20%28single-precision%29))
  (bind _output (Utilities|ApplyValueatFPS 1.0))
  (bind _output_2 (Utilities|ApplyValueatFPS -1.0))
  (bind _switch (Variables|Default|GetSwitch))
  (bind _switch_2 (Variables|Default|GetSwitch))
  (bind _returnvalue (Transformation|GetWorldLocation _switch_2))
  (bind _returnvalue_2 (Transformation|GetWorldLocation _switch))
  (bind _returnvalue_3 (+ (.z _returnvalue_2) _output))
  (bind _returnvalue_4 (+ (.z _returnvalue) _output_2))
  (if (Variables|Default|GetIsSwitchOnObject)
    (Transformation|SetWorldLocation (Variables|Default|GetSwitch) (Math|Vector|MakeVector (.x _returnvalue) (.y _returnvalue) _returnvalue_4) false false)
    (if (<= _returnvalue_4 (- (.z (Variables|Default|GetStartVector)) 25.0))
      (Variables|Default|SetIsSwitchOnObject false)
      (CallFunction|SwitchonObject))
    (elif (Variables|Default|GetIsPressureSensitive)
      (if (not (Variables|Default|GetIsOnActor))
        (Transformation|SetWorldLocation (Variables|Default|GetSwitch) (Math|Vector|MakeVector (.x _returnvalue_2) (.y _returnvalue_2) _returnvalue_3) false false)
        (if (> _returnvalue_3 (.z (Variables|Default|GetStartVector)))
          (Variables|Default|SetIsOnActor true))))))

(fn ConstructionScript)