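; CureObject_BP is a healing actor that IsItem switches between a one-shot pickup and a healing area.
; As an item it shows a cube and, on player overlap, restores full Life, plays a sound and destroys itself.
; As an area it shows particles, fades a looping-area sound with overlap, and heals every Tick through negative Damage.
; Box overlaps also toggle the player's IsOnCure flag, which gates that healing.
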(event OnComponentBeginOverlap(Box)
  (params (OverlappedComponent :type Primitive%20Component%20Object%20Reference) (OtherActor :type Actor%20Object%20Reference) (OtherComp :type Primitive%20Component%20Object%20Reference) (OtherBodyIndex :type Integer) (bFromSweep :type Boolean) (SweepResult :type Hit%20Result%20Structure%20%28by%20ref%29))
  (bind (_asplayer_bp _bsuccess) (Utilities|Casting|CastToPlayer_BP OtherActor))
  (if _bsuccess
    (Variables|/Game/Content/Blueprint/Player/Player_BP.Player_BP_C|SetIsOnCure _asplayer_bp true)
    (if (Variables|Default|GetIsItem)
      (Variables|/Game/Content/Blueprint/Player/Player_BP.Player_BP_C|SetLife _asplayer_bp (Variables|/Game/Content/Blueprint/Player/Player_BP.Player_BP_C|GetMaxLife _asplayer_bp))
      (Default|Damage _asplayer_bp 0.0)
      (Audio|PlaySound2D "/Game/Content/Sound/SE/SE/heel_item.heel_item" 1.0 1.0 0.0 0 0)
      (Actor|DestroyActor)
      (else
        (Audio|Components|Audio|FadeIn (Variables|Default|GetHeelArea) 0.5 0.7 0.0 "Linear" :!class /Script/Engine.AudioComponent)))))

(event OnComponentEndOverlap(Box)
  (params (OverlappedComponent :type Primitive%20Component%20Object%20Reference) (OtherActor :type Actor%20Object%20Reference) (OtherComp :type Primitive%20Component%20Object%20Reference) (OtherBodyIndex :type Integer))
  (bind (_asplayer_bp _bsuccess) (Utilities|Casting|CastToPlayer_BP OtherActor))
  (if _bsuccess
    (Variables|/Game/Content/Blueprint/Player/Player_BP.Player_BP_C|SetIsOnCure _asplayer_bp false)
    (if (not (Variables|Default|GetIsItem))
      (Audio|Components|Audio|FadeOut (Variables|Default|GetHeelArea) 0.5 0.0 "Linear" :!class /Script/Engine.AudioComponent))))

(event EventBeginPlay
  (if (Variables|Default|GetIsItem)
    (Rendering|SetVisibility (Variables|Default|GetParticleSystem) false false)
    (else
      (Rendering|SetVisibility (Variables|Default|GetCube) false false)
      (bind _returnvalue (Audio|SpawnSound2D "/Game/Content/Sound/SE/SE/heel_Area.heel_Area" 0.5 1.0 0.0 0 false false))
      (bind _output_get (Variables|Default|SetHeelArea _returnvalue))
      (Audio|Components|Audio|Stop _output_get))))

(event Collision|EventActorBeginOverlap
  (params (OtherActor :type Actor%20Object%20Reference)))

(event EventTick
  (params (DeltaSeconds :type Float%20%28single-precision%29))
  (for _array_element (Collision|GetOverlappingActors (Variables|Default|GetBox) "/Game/Content/Blueprint/Player/Player_BP.Player_BP_C" :!class /Script/Engine.PrimitiveComponent)
    (bind _asplayer_bp (Utilities|Casting|CastToPlayer_BP _array_element))
    (if (Variables|/Game/Content/Blueprint/Player/Player_BP.Player_BP_C|GetIsOnCure _asplayer_bp)
      (if (not (Variables|Default|GetIsItem))
        (if (< (Variables|/Game/Content/Blueprint/Player/Player_BP.Player_BP_C|GetLife _asplayer_bp) (Variables|/Game/Content/Blueprint/Player/Player_BP.Player_BP_C|GetMaxLife _asplayer_bp))
          (Default|Damage _asplayer_bp (* (Variables|Default|GetCureValue) -1.0))
          (else
            (Variables|/Game/Content/Blueprint/Player/Player_BP.Player_BP_C|SetLife _asplayer_bp (Variables|/Game/Content/Blueprint/Player/Player_BP.Player_BP_C|GetMaxLife _asplayer_bp))))))))

(fn ConstructionScript)