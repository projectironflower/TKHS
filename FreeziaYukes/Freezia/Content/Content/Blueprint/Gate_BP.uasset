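; Double-door gate actor that swings open or closed when its GateOpen or GateClose events are called.
; Those events set opposing flags, and Tick yaws the left and right axes in opposite directions at separate open and close speeds, using ApplyValueAtFPS for each step.
; An accumulated rotation value stops motion at the open limit or at zero, where GateClosed is called once closing finishes.
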(event Custom|GateOpen
  (Variables|Default|SetIsClose false)
  (Variables|Default|SetIsOpen true))

(event Custom|GateClose
  (Variables|Default|SetIsOpen false)
  (Variables|Default|SetIsClose true))

(event EventBeginPlay)

(event Collision|EventActorBeginOverlap
  (params (OtherActor :type Actor%20Object%20Reference)))

(event EventTick
  (params (DeltaSeconds :type Float%20%28single-precision%29))
  (bind _leftaxis (Variables|Default|GetLeftAxis))
  (bind _rightaxis (Variables|Default|GetRightAxis))
  (bind _leftaxis_2 (Variables|Default|GetLeftAxis))
  (bind _rightaxis_2 (Variables|Default|GetRightAxis))
  (bind _returnvalue (Transformation|GetWorldRotation _leftaxis_2))
  (bind _returnvalue_2 (Transformation|GetWorldRotation _rightaxis_2))
  (bind _returnvalue_3 (Transformation|GetWorldRotation _rightaxis))
  (bind _returnvalue_4 (Transformation|GetWorldRotation _leftaxis))
  (if (Variables|Default|GetIsOpen)
    (Transformation|SetWorldRotation _leftaxis_2 (Math|Rotator|MakeRotator (.roll _returnvalue) (.pitch _returnvalue) (+ (.yaw _returnvalue) (Utilities|ApplyValueatFPS (Variables|Default|GetOpenSpeed)))) false true)
    (Transformation|SetWorldRotation _rightaxis_2 (Math|Rotator|MakeRotator (.roll _returnvalue_2) (.pitch _returnvalue_2) (- (.yaw _returnvalue_2) (Utilities|ApplyValueatFPS (Variables|Default|GetOpenSpeed)))) false true)
    (bind _output_get (Variables|Default|SetRotateValue (+ (Variables|Default|GetRotateValue) (Utilities|ApplyValueatFPS (Variables|Default|GetOpenSpeed)))))
    (if (>= _output_get (Variables|Default|GetRotateLimit))
      (Variables|Default|SetIsOpen false)
      (Variables|Default|SetRotateValue (Variables|Default|GetRotateLimit)))
    (elif (Variables|Default|GetIsClose)
      (Transformation|SetWorldRotation _leftaxis (Math|Rotator|MakeRotator (.roll _returnvalue_4) (.pitch _returnvalue_4) (- (.yaw _returnvalue_4) (Utilities|ApplyValueatFPS (Variables|Default|GetCloseSpeed)))) false true)
      (Transformation|SetWorldRotation _rightaxis (Math|Rotator|MakeRotator (.roll _returnvalue_3) (.pitch _returnvalue_3) (+ (.yaw _returnvalue_3) (Utilities|ApplyValueatFPS (Variables|Default|GetCloseSpeed)))) false true)
      (bind _output_get_2 (Variables|Default|SetRotateValue (- (Variables|Default|GetRotateValue) (Utilities|ApplyValueatFPS (Variables|Default|GetCloseSpeed)))))
      (if (<= _output_get_2 0.0)
        (Variables|Default|SetIsClose false)
        (Variables|Default|SetRotateValue 0.0)
        (Default|CallGateClosed)))))

(fn ConstructionScript)