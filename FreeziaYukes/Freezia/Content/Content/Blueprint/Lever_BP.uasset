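; Lever actor that switches linked level objects when the player touches it.
; Overlap by Player_BP while active flips its flag, plays a sound and, after a delay, runs SetObjectActive and CallMoveLever.
; SetObjectActive toggles each SetObject entry between Start and Stop using its IsActive or IsFire state.
; Tick swings the lever rod toward the flag's position at frame-rate-scaled speed, and Reset restores the flag.
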(event OnComponentBeginOverlap(Collision)
  (params (OverlappedComponent :type Primitive%20Component%20Object%20Reference) (OtherActor :type Actor%20Object%20Reference) (OtherComp :type Primitive%20Component%20Object%20Reference) (OtherBodyIndex :type Integer) (bFromSweep :type Boolean) (SweepResult :type Hit%20Result%20Structure%20%28by%20ref%29))
  ;[1 1 1] オブジェクトのオンオフ切り替え処理
  (if (.bSuccess (Utilities|Casting|CastToPlayer_BP OtherActor))
    (if (Variables|Default|GetObjectDefaltIsActive)
      (Variables|Default|SetObjectDefaltIsActive false)
      (Audio|PlaySoundatLocation 0 (Transformation|GetWorldLocation (Variables|Default|GetLever_main)) "0, 0, 0" 1.0 1.0 0.0 0 0 0)
      (Utilities|FlowControl|Delay 1.3)
      (CallFunction|SetObjectActive)
      (Default|CallMoveLever))))

(event Custom|Reset
  (bind _lever_bou (Variables|Default|GetLever_bou))
  (bind _returnvalue (Transformation|GetWorldRotation _lever_bou))
  (bind (_roll _pitch _yaw) (Math|Rotator|BreakRotator _returnvalue))
  (Variables|Default|SetObjectDefaltIsActive true)
  (if (<= _roll 0.0)
    (Transformation|SetWorldRotation _lever_bou (Math|Rotator|MakeRotator (+ _roll 2.0) _pitch _yaw) false false)))

(event EventBeginPlay)

(event Collision|EventActorBeginOverlap
  (params (OtherActor :type Actor%20Object%20Reference)))

(event EventTick
  (params (DeltaSeconds :type Float%20%28single-precision%29))
  (bind _lever_bou (Variables|Default|GetLever_bou))
  (bind _lever_bou_2 (Variables|Default|GetLever_bou))
  (bind _returnvalue (Transformation|GetWorldRotation _lever_bou_2))
  (bind _returnvalue_2 (Transformation|GetWorldRotation _lever_bou))
  (bind (_roll _pitch _yaw) (Math|Rotator|BreakRotator _returnvalue))
  (bind (_roll_2 _pitch_2 _yaw_2) (Math|Rotator|BreakRotator _returnvalue_2))
  ;[1 1 1] レバーが動く処理
  (if (Variables|Default|GetObjectDefaltIsActive)
    (if (<= _roll_2 0.0)
      (Transformation|SetWorldRotation _lever_bou (Math|Rotator|MakeRotator (+ _roll_2 (* (/ DeltaSeconds (/ 1.0 6e+01)) 3.5)) _pitch_2 _yaw_2) false false))
    (elif (>= _roll -1.5e+02)
      (Transformation|SetWorldRotation _lever_bou_2 (Math|Rotator|MakeRotator (+ _roll (* (/ DeltaSeconds (/ 1.0 6e+01)) -3.5)) _pitch _yaw) false false))))

(fn ConstructionScript)

(fn SetObjectActive
  (for _array_element (Variables|Default|GetSetObject)
    (bind _aspress_machine_bp (Utilities|Casting|CastTo _array_element)
      (:then
        (if (Variables|Default|GetIsActive _aspress_machine_bp)
          (CallFunction|Stop _aspress_machine_bp)
          (else
            (CallFunction|Start _aspress_machine_bp))))
      (:CastFailed
        (bind _asburner_bp (Utilities|Casting|CastTo _array_element))
        (if (Variables|Default|GetIsFire _asburner_bp)
          (CallFunction|Stop _asburner_bp)
          (else
            (CallFunction|Start _asburner_bp)))))))