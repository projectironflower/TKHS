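; CheckPoint_BP is a checkpoint actor that updates the player's respawn point when touched.
; When a Player_BP overlaps its Box, it passes a location offset and its checkpoint number to GameMode_BP through SetRespawnOffset.
; The offset runs from the first PlayerStart found in the level to a point slightly above the checkpoint, so it is relative rather than a world position.
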(event OnComponentBeginOverlap(Box)
  (params (OverlappedComponent :type Primitive%20Component%20Object%20Reference) (OtherActor :type Actor%20Object%20Reference) (OtherComp :type Primitive%20Component%20Object%20Reference) (OtherBodyIndex :type Integer) (bFromSweep :type Boolean) (SweepResult :type Hit%20Result%20Structure%20%28by%20ref%29))
  (Utilities|Casting|CastToPlayer_BP OtherActor)
  (bind _asgame_mode_bp (Utilities|Casting|CastToGameMode_BP (Game|GetGameMode)))
  (bind _outactors (Actor|GetAllActorsOfClass "/Script/Engine.PlayerStart"))
  (Default|SetRespawnOffset _asgame_mode_bp (- (+ (Transformation|GetActorLocation) "0, 0,100.000000") (Transformation|GetActorLocation (Utilities|Array|Get(acopy) _outactors))) (Variables|Default|GetCheckPointNum)))

(event EventBeginPlay)

(event Collision|EventActorBeginOverlap
  (params (OtherActor :type Actor%20Object%20Reference)))

(event EventTick
  (params (DeltaSeconds :type Float%20%28single-precision%29)))

(fn ConstructionScript)