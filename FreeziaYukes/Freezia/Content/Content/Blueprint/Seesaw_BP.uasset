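; Seesaw actor that tilts under a sufficiently heavy, jump-ready player inside its Box and resets its transform on GameMode respawn.
; Each Tick it adds delta-time-scaled roll based on the player's world Y offset from the pivot and their mass.
; Roll stops at angle limits or when the descending side's box overlaps a step-up component.
; The construction script shifts the mesh and side boxes by OffCenter to move the pivot.
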(event Custom|ResetTrasform
  (Transformation|SetActorTransform (Variables|Default|GetBaseTransform)))

(event EventBeginPlay
  (Variables|Default|SetBaseTransform (Transformation|GetActorTransform))
  (bind _asgame_mode_bp (Utilities|Casting|CastToGameMode_BP (Game|GetGameMode)))
  (EventDispatchers|BindEventtoOnRespawn _asgame_mode_bp (delegate Custom|ResetTrasform)))

(event Collision|EventActorBeginOverlap
  (params (OtherActor :type Actor%20Object%20Reference)))

(event EventTick
  (params (DeltaSeconds :type Float%20%28single-precision%29))
  (Variables|Default|SetEnableRotate true)
  (for _array_element (Collision|GetOverlappingActors (Variables|Default|GetBox) "/Game/Content/Blueprint/Player/Player_BP.Player_BP_C" :!class /Script/Engine.PrimitiveComponent)
    (bind _asplayer_bp (Utilities|Casting|CastToPlayer_BP _array_element))
    (if (Character|CanJump _asplayer_bp)
      (if (> (/ (Variables|/Script/Engine.CharacterMovementComponent|GetMass (Variables|/Script/Engine.Character|GetCharacterMovement _asplayer_bp)) (Variables|/Game/Content/Blueprint/Player/Player_BP.Player_BP_C|GetMaxMass _asplayer_bp)) (Variables|Default|GetMaxMassRatio))
        (CallFunction|Rotation (Transformation|GetWorldLocation (Variables|/Script/Engine.Character|GetCapsuleComponent _asplayer_bp)) (Variables|/Script/Engine.CharacterMovementComponent|GetMass (Variables|/Script/Engine.Character|GetCharacterMovement _asplayer_bp)))))))

(fn ConstructionScript
  (bind _offcenter (Variables|Default|GetOffCenter))
  (bind _returnvalue (* _offcenter -1.0))
  (Transformation|SetRelativeLocation (Variables|Default|GetStaticMesh) _returnvalue false false)
  (Transformation|SetRelativeLocation (Variables|Default|GetBoxLeft) (+ _returnvalue (Variables|/Script/Engine.SceneComponent|GetRelativeLocation (Variables|Default|GetBoxLeft))) false false)
  (Transformation|SetRelativeLocation (Variables|Default|GetBoxRight) (+ _returnvalue (Variables|/Script/Engine.SceneComponent|GetRelativeLocation (Variables|Default|GetBoxRight))) false false))

(fn Rotation
  (params (PlayerPosition :type Vector) (PlayerMass :type Float%20%28single-precision%29))
  (bind _y (Math|Vector|BreakVector PlayerPosition))
  (bind _defaultsceneroot (Variables|Default|GetDefaultSceneRoot))
  (bind _returnvalue (Transformation|GetWorldLocation _defaultsceneroot))
  (bind _returnvalue_2 (Transformation|GetWorldRotation _defaultsceneroot))
  (bind (_roll _pitch _yaw) (Math|Rotator|BreakRotator _returnvalue_2))
  (bind _y_2 (Math|Vector|BreakVector _returnvalue))
  (bind _returnvalue_3 (- _y _y_2))
  (CallFunction|CulcEnableRotate _returnvalue_3)
  (if (Variables|Default|GetEnableRotate)
    (Transformation|SetWorldRotation (Variables|Default|GetDefaultSceneRoot) (Math|Rotator|MakeRotator (+ (* (* _returnvalue_3 PlayerMass (Variables|Default|GetRotSpeed) (Variables|Default|GetRotCoefficient)) (Utilities|Time|GetWorldDeltaSeconds) 6e+01) _roll) _pitch _yaw) false false)))

(fn CulcEnableRotate
  (params (Position :type Float%20%28single-precision%29))
  (bind _returnvalue (Game|Player|GetPlayerPawn 0))
  (bind _defaultsceneroot (Variables|Default|GetDefaultSceneRoot))
  (bind _returnvalue_2 (Transformation|GetWorldRotation _defaultsceneroot))
  (bind _roll (Math|Rotator|BreakRotator _returnvalue_2))
  (if (< Position 0.0)
    (if (<= _roll (Variables|Default|GetMinRot))
      (Variables|Default|SetEnableRotate false)
      (else
        (for _array_element (Class|PrimitiveComponent|GetOverlappingComponents (Variables|Default|GetBoxLeft))
          (if (Class|PrimitiveComponent|CanCharacterStepUp _array_element _returnvalue)
            (Variables|Default|SetEnableRotate false)))))
    (elif (> Position 0.0)
      (if (>= _roll (Variables|Default|GetMaxRot))
        (Variables|Default|SetEnableRotate false)
        (else
          (for _array_element_2 (Class|PrimitiveComponent|GetOverlappingComponents (Variables|Default|GetBoxRight))
            (if (Class|PrimitiveComponent|CanCharacterStepUp _array_element_2 _returnvalue)
              (Variables|Default|SetEnableRotate false))))))))

(fn Reset
  (Transformation|SetWorldRotation (Variables|Default|GetDefaultSceneRoot) "0, 0, 0" false false))