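; Result billboard actor that takes over the view when the goal trigger fires its player event.
; On BeginPlay it binds to the level's Goal_Trigger_BP and creates a result widget through a level-name switch, whose only branch currently makes the Pause widget.
; When triggered, it blends the camera to itself, prints the time since its creation as the clear time, and shows the widget on its widget component.
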(event Custom|GetClearTime
  (Game|Player|SetViewTargetwithBlend (Game|GetPlayerController 0) self 1.5 "VTBlend_Cubic" 0.0 false)
  (Development|PrintString (Class|KismetStringLibrary|TimeSecondstoString (Actor|GetGameTimeSinceCreation)))
  (UserInterface|SetWidget (Variables|Default|GetWidget) (Variables|Default|GetResultWidget)))

(event EventBeginPlay
  (bind _returnvalue (Actor|GetActorOfClass "/Game/Content/Blueprint/Goal_Trigger_BP.Goal_Trigger_BP_C"))
  (EventDispatchers|BindEventtoOnPlayer _returnvalue (delegate Custom|GetClearTime))
  (bind _returnvalue_2 (Game|GetCurrentLevelName true))
  (switch string _returnvalue_2
    (:Default
      (bind _returnvalue_3 (UserInterface|CreateWidget "/Game/Content/UI/Pause.Pause_C"))
      (Variables|Default|SetResultWidget _returnvalue_3))))

(event Collision|EventActorBeginOverlap
  (params (OtherActor :type Actor%20Object%20Reference)))

(event EventTick
  (params (DeltaSeconds :type Float%20%28single-precision%29)))

(fn ConstructionScript)