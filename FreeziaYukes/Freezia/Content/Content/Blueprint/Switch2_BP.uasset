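; Floor switch actor that sinks under the player or a MovableBlock_BP and opens the Gate_BP actors in SetObjects.
; Box overlaps and a per-tick block check set state flags that drive the switch mesh down a short, frame-rate-scaled distance before opening gates.
; A raise-and-close path runs only for overlapping blocks whose MeshCollision leaves the box; the player leaving just clears the on flag.
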(event OnComponentBeginOverlap(Box)
  (params (OverlappedComponent :type Primitive%20Component%20Object%20Reference) (OtherActor :type Actor%20Object%20Reference) (OtherComp :type Primitive%20Component%20Object%20Reference) (OtherBodyIndex :type Integer) (bFromSweep :type Boolean) (SweepResult :type Hit%20Result%20Structure%20%28by%20ref%29))
  (Utilities|Casting|CastToPlayer_BP OtherActor)
  (Variables|Default|SetIsSwitchOnObject true))

(event OnComponentEndOverlap(Box)
  (params (OverlappedComponent :type Primitive%20Component%20Object%20Reference) (OtherActor :type Actor%20Object%20Reference) (OtherComp :type Primitive%20Component%20Object%20Reference) (OtherBodyIndex :type Integer))
  (bind _asplayer_bp (Utilities|Casting|CastToPlayer_BP OtherActor))
  (if (not (Collision|IsOverlappingActor (Variables|Default|GetBox) _asplayer_bp :!class /Script/Engine.PrimitiveComponent))
    (Variables|Default|SetIsSwitchOn false)))

(event Custom|SwitchOnObject
  (for _array_element (Variables|Default|GetSetObjects)
    (bind _asgate_bp (Utilities|Casting|CastToGate_BP _array_element))
    (Default|GateOpen _asgate_bp)))

(event Custom|SwitchOutObject
  (for _array_element (Variables|Default|GetSetObjects)
    (bind _asgate_bp (Utilities|Casting|CastToGate_BP _array_element))
    (Default|GateClose _asgate_bp)))

(event EventBeginPlay
  (Variables|Default|SetStartVector (Transformation|GetWorldLocation (Variables|Default|GetSwitch))))

(event Collision|EventActorBeginOverlap
  (params (OtherActor :type Actor%20Object%20Reference)))

(event EventTick
  (params (DeltaSeconds :type Float%20%28single-precision%29))
  (CallFunction|IsonMovableBlock))

(fn ConstructionScript)

(fn IsonMovableBlock
  (bind _output (Utilities|ApplyValueatFPS 1.0))
  (bind _switch (Variables|Default|GetSwitch))
  (bind _box (Variables|Default|GetBox))
  (bind _returnvalue (Transformation|GetWorldLocation _switch))
  (bind _returnvalue_2 (+ (.z _returnvalue) _output))
  (if (Variables|Default|GetIsSwitchOnObject)
    (CallFunction|NewFunction0)
    (elif (Variables|Default|GetIsSwitchOn)
      (bind _array_element (Utilities|Array|ForEachLoopwithBreak (Collision|GetOverlappingActors (Variables|Default|GetBox) "/Game/Content/Blueprint/MovableBlock_BP.MovableBlock_BP_C" :!class /Script/Engine.PrimitiveComponent))
        (:LoopBody
          (if (.bSuccess (Utilities|Casting|CastToMovableBlock_BP _array_element))
            (if (not (Class|PrimitiveComponent|IsOverlappingComponent (Variables|/Game/Content/Blueprint/MovableBlock_BP.MovableBlock_BP_C|GetMeshCollision (.AsMovable%20Block%20BP (Utilities|Casting|CastToMovableBlock_BP _array_element))) _box))
              (Transformation|SetWorldLocation (Variables|Default|GetSwitch) (Math|Vector|MakeVector (.x _returnvalue) (.y _returnvalue) _returnvalue_2) false false)
              (if (> _returnvalue_2 (.z (Variables|Default|GetStartVector)))
                (Variables|Default|SetIsSwitchOn false)
                (CallFunction|SwitchOutObject))))))
      (else
        (bind _outactors (Actor|GetAllActorsOfClass "/Game/Content/Blueprint/MovableBlock_BP.MovableBlock_BP_C"))
        (for _array_element_2 _outactors
          (if (.bSuccess (Utilities|Casting|CastToMovableBlock_BP _array_element_2))
            (if (Class|PrimitiveComponent|IsOverlappingComponent (Variables|/Game/Content/Blueprint/MovableBlock_BP.MovableBlock_BP_C|GetMeshCollision (.AsMovable%20Block%20BP (Utilities|Casting|CastToMovableBlock_BP _array_element_2))) _box)
              (Variables|Default|SetIsSwitchOnObject true)
              (else
                (Variables|Default|SetIsOnActor false)))))
        (return)))))

(fn NewFunction0
  (bind _output (Utilities|ApplyValueatFPS -1.0))
  (bind _switch (Variables|Default|GetSwitch))
  (bind _returnvalue (Transformation|GetWorldLocation _switch))
  (bind _returnvalue_2 (+ (.z _returnvalue) _output))
  (if (< _returnvalue_2 (- (.z (Variables|Default|GetStartVector)) (Utilities|ApplyValueatFPS 25.0)))
    (Variables|Default|SetIsSwitchOn true)
    (Variables|Default|SetIsSwitchOnObject false)
    (CallFunction|SwitchonObject)
    (else
      (Transformation|SetWorldLocation (Variables|Default|GetSwitch) (Math|Vector|MakeVector (.x _returnvalue) (.y _returnvalue) _returnvalue_2) false false))))