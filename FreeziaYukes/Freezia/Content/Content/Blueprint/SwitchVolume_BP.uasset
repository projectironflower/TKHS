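; SwitchVolume_BP is a volume that turns the player's mesh onto one of six configurable headings, apparently branching paths, from movement input.
; Each Tick it checks whether the player's box overlaps its own and, if the player can jump, calls SwitchDirection.
; Forward-axis sign and vertical axis (up, neutral, down) pick the heading.
; GetYaw offsets left headings by 180 degrees, adding another 180 when the player's CheckReverse is true.
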(event EventBeginPlay)

(event Collision|EventActorBeginOverlap
  (params (OtherActor :type Actor%20Object%20Reference)))

(event EventTick
  (params (DeltaSeconds :type Float%20%28single-precision%29))
  (bind _isoverlapping (CallFunction|IsOverlappingPlayer))
  (if _isoverlapping
    (bind _asplayer_bp (Utilities|Casting|CastToPlayer_BP (Game|Player|GetPlayerPawn 0)))
    (if (Character|CanJump _asplayer_bp)
      (CallFunction|SwitchDirection (Variables|/Game/Content/Blueprint/Player/Player_BP.Player_BP_C|GetAxisVertical _asplayer_bp)))))

(fn ConstructionScript)

(fn IsOverlappingPlayer
  (bind _asplayer_bp (Utilities|Casting|CastToPlayer_BP (Game|Player|GetPlayerPawn 0))
    (:then
      (return (Class|PrimitiveComponent|IsOverlappingComponent (Variables|/Game/Content/Blueprint/Player/Player_BP.Player_BP_C|GetBox _asplayer_bp) (Variables|Default|GetBox))))
    (:CastFailed
      (return false))))

(fn SwitchDirection
  (params (AxisVertical :type Float%20%28single-precision%29))
  ;[1 1 1] 軸値の保存
  (LocalVariables|SetAxisValue AxisVertical)
  ;[1 1 1] プレイヤーの向き判別
  (bind _asplayer_bp (Utilities|Casting|CastToPlayer_BP (Game|Player|GetPlayerPawn 0)))
  (LocalVariables|SetPlayer _asplayer_bp)
  (if (> (Variables|/Game/Content/Blueprint/Player/Player_BP.Player_BP_C|GetAxisForword _asplayer_bp) 0.0) ; 進行方向右向き
    ;[1 1 1] 軸値で場合分け
    (if (> (LocalVariables|GetAxisValue) 0.0)
      ;[1 1 1] プレイヤーを回転
      (CallFunction|RotatePlayer (LocalVariables|GetPlayer) 0 (Utilities|CheckReverse _asplayer_bp (Variables|/Game/Content/Blueprint/Player/Player_BP.Player_BP_C|GetAxisForword _asplayer_bp)))
      (elif (< (LocalVariables|GetAxisValue) 0.0)
        (CallFunction|RotatePlayer (LocalVariables|GetPlayer) 2 (Utilities|CheckReverse _asplayer_bp (Variables|/Game/Content/Blueprint/Player/Player_BP.Player_BP_C|GetAxisForword _asplayer_bp)))
        (else
          (CallFunction|RotatePlayer (LocalVariables|GetPlayer) 1 (Utilities|CheckReverse _asplayer_bp (Variables|/Game/Content/Blueprint/Player/Player_BP.Player_BP_C|GetAxisForword _asplayer_bp))))))
    (return)
    (elif (< (Variables|/Game/Content/Blueprint/Player/Player_BP.Player_BP_C|GetAxisForword _asplayer_bp) 0.0) ; 進行方向左向き
      (if (> (LocalVariables|GetAxisValue) 0.0)
        (CallFunction|RotatePlayer (LocalVariables|GetPlayer) 3 (Utilities|CheckReverse _asplayer_bp (Variables|/Game/Content/Blueprint/Player/Player_BP.Player_BP_C|GetAxisForword _asplayer_bp)))
        (elif (< (LocalVariables|GetAxisValue) 0.0)
          (CallFunction|RotatePlayer (LocalVariables|GetPlayer) 5 (Utilities|CheckReverse _asplayer_bp (Variables|/Game/Content/Blueprint/Player/Player_BP.Player_BP_C|GetAxisForword _asplayer_bp)))
          (else
            (CallFunction|RotatePlayer (LocalVariables|GetPlayer) 4 (Utilities|CheckReverse _asplayer_bp (Variables|/Game/Content/Blueprint/Player/Player_BP.Player_BP_C|GetAxisForword _asplayer_bp))))))
      (return))))

(fn RotatePlayer
  (params (Player :type Player%20BP%20Object%20Reference) (Puttern :type Integer) (IsReverse :type Boolean))
  (bind _yaw (CallFunction|GetYaw Puttern IsReverse))
  (Transformation|SetWorldRotation (Variables|/Script/Engine.Character|GetMesh Player) (Math|Rotator|MakeRotator 0.0 0.0 _yaw) false false))

(fn GetYaw
  (params (NewParam :type Integer) (IsReverse :type Boolean))
  (bind _righttopdegree (Variables|Default|GetRightTopDegree))
  (bind _rightdegree (Variables|Default|GetRightDegree))
  (bind _rightbotdegree (Variables|Default|GetRightBotDegree))
  (bind _lefttopdegree (Variables|Default|GetLeftTopDegree))
  (bind _leftdegree (Variables|Default|GetLeftDegree))
  (bind _leftbotdegree (Variables|Default|GetLeftBotDegree))
  (bind _returnvalue (+ _leftdegree 1.8e+02))
  (bind _returnvalue_2 (+ _lefttopdegree 1.8e+02))
  (bind _returnvalue_3 (+ _leftbotdegree 1.8e+02))
  (bind _array (Utilities|Array|MakeArray _righttopdegree _rightdegree _rightbotdegree _returnvalue_2 _returnvalue _returnvalue_3))
  (bind _output (Utilities|Array|Get(acopy) _array NewParam))
  (if IsReverse
    (return (+ _output 1.8e+02))
    (else
      (return _output))))