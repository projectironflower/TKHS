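; Conveyor belt actor that carries the player sideways along the Y axis while they stand on it.
; Box overlap events flag when the player is on the belt.
; While flagged and the player is alive, Tick moves the pawn with a swept, delta-time-scaled offset based on MoveSpeed and the ToRight direction.
; The construction script sets the mesh material's Speed vector from the same direction and speed.
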(event OnComponentBeginOverlap(Box)
  (params (OverlappedComponent :type Primitive%20Component%20Object%20Reference) (OtherActor :type Actor%20Object%20Reference) (OtherComp :type Primitive%20Component%20Object%20Reference) (OtherBodyIndex :type Integer) (bFromSweep :type Boolean) (SweepResult :type Hit%20Result%20Structure%20%28by%20ref%29))
  (Utilities|Casting|CastToPlayer_BP OtherActor)
  (Variables|Default|SetIsOnPlayer true))

(event OnComponentEndOverlap(Box)
  (params (OverlappedComponent :type Primitive%20Component%20Object%20Reference) (OtherActor :type Actor%20Object%20Reference) (OtherComp :type Primitive%20Component%20Object%20Reference) (OtherBodyIndex :type Integer))
  (Utilities|Casting|CastToPlayer_BP OtherActor)
  (Variables|Default|SetIsOnPlayer false))

(event EventBeginPlay)

(event Collision|EventActorBeginOverlap
  (params (OtherActor :type Actor%20Object%20Reference)))

(event EventTick
  (params (DeltaSeconds :type Float%20%28single-precision%29))
  (bind _returnvalue (Game|Player|GetPlayerPawn 0))
  (bind _movespeed (Variables|Default|GetMoveSpeed))
  (bind _constant (Variables|Default|GetConstant))
  (bind _returnvalue_2 (Transformation|GetActorLocation _returnvalue))
  (bind _returnvalue_3 (* DeltaSeconds _movespeed _constant 6e+01))
  (if (Variables|Default|GetIsOnPlayer)
    (bind _asplayer_bp (Utilities|Casting|CastToPlayer_BP _returnvalue))
    (if (not (Variables|/Game/Content/Blueprint/Player/Player_BP.Player_BP_C|GetIsDead _asplayer_bp))
      (if (Variables|Default|GetToRight)
        (Transformation|SetActorLocation _returnvalue (+ _returnvalue_2 (* "0,4.800000,0.000000" _returnvalue_3)) true false)
        (else
          (Transformation|SetActorLocation _returnvalue (+ _returnvalue_2 (* "0,-4.800000, 0" _returnvalue_3)) true false))))))

(fn ConstructionScript
  (bind _movespeed (Variables|Default|GetMoveSpeed))
  (bind _staticmesh (Variables|Default|GetStaticMesh))
  (bind _returnvalue (/ _movespeed 0.5))
  (if (Variables|Default|GetToRight)
    (Rendering|Material|SetVectorParameterValueonMaterials _staticmesh "Speed" (* "1.000000, 0, 0" _returnvalue))
    (else
      (Rendering|Material|SetVectorParameterValueonMaterials _staticmesh "Speed" (* "-1.000000, 0, 0" _returnvalue)))))