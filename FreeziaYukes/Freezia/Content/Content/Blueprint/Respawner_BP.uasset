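; Respawner actor that recreates a referenced actor after it is destroyed, using the respawner's own transform.
; On BeginPlay it caches the actor's class and binds to its destroyed event, which only sets a pending-respawn flag.
; A separate Respawn event, not called within this Blueprint, checks the flag, waits briefly, spawns the class, rebinds the destroyed event and clears the flag.
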(event Custom|Respawn
  (if (Variables|Default|GetIsRespawn)
    (Utilities|FlowControl|Delay 0.01)
    (bind _returnvalue (Game|SpawnActorfromClass (Variables|Default|GetRespawnActorClass) (Transformation|GetActorTransform) "Undefined" 0 0))
    (Game|BindEventtoOnDestroyed _returnvalue (delegate Custom|SetRespawn))
    (Variables|Default|SetIsRespawn false)))

(event Custom|SetRespawn
  (params (DestroyedActor :type Actor%20Object%20Reference))
  (Variables|Default|SetIsRespawn true))

(event EventBeginPlay
  (bind _actor (Variables|Default|GetActor))
  (Variables|Default|SetRespawnActorClass (Utilities|GetClass _actor))
  (Game|BindEventtoOnDestroyed _actor (delegate Custom|SetRespawn)))

(event Collision|EventActorBeginOverlap
  (params (OtherActor :type Actor%20Object%20Reference)))

(event EventTick
  (params (DeltaSeconds :type Float%20%28single-precision%29)))

(fn ConstructionScript)