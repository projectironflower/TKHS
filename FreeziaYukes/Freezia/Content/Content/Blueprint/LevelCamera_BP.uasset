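; LevelCamera_BP is a level camera actor that becomes the player's view and can follow the Player_BP pawn along two axes.
; On BeginPlay it moves to the world origin, then after a short delay blends the first player controller's view target to itself.
; While IsSync is true, Tick copies the pawn's Y and Z with a fixed upward offset and keeps its own X, with no smoothing.
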(event EventBeginPlay
  (Transformation|SetActorLocation "0, 0, 0" false false)
  (Utilities|FlowControl|Delay 0.2)
  (Game|Player|SetViewTargetwithBlend (Game|GetPlayerController 0) self 0.1 "VTBlend_Linear" 0.0 false))

(event Collision|EventActorBeginOverlap
  (params (OtherActor :type Actor%20Object%20Reference)))

(event EventTick
  (params (DeltaSeconds :type Float%20%28single-precision%29))
  (if (Variables|Default|GetIsSync)
    (bind _asplayer_bp (Utilities|Casting|CastToPlayer_BP (Game|Player|GetPlayerPawn 0)))
    (Transformation|SetActorLocation (Math|Vector|MakeVector (.X (Math|Vector|BreakVector (Transformation|GetActorLocation))) (.Y (Math|Vector|BreakVector (Transformation|GetActorLocation _asplayer_bp))) (+ (.Z (Math|Vector|BreakVector (Transformation|GetActorLocation _asplayer_bp))) 1e+02)) false false)))

(fn ConstructionScript)