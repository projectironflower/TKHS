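; BGMPlayer_BP is a Blueprint that plays the background music for the current stage.
; On BeginPlay, Init picks one of six BGM cues by matching the current level name, then starts playback.
; It binds StopBGM to the player pawn's stop-BGM event and PlayBGM to the game mode's respawn event, so music restarts from the beginning on respawn.
; Pause and Restart events toggle the paused state.
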(event Custom|Pause
  (Class|AudioComponent|SetPaused (Variables|Default|GetBGM) true))

(event Custom|StopBGM
  (Audio|Components|Audio|Stop (Variables|Default|GetBGM)))

(event Custom|Restart
  (Class|AudioComponent|SetPaused (Variables|Default|GetBGM) false))

(event Custom|PlayBGM
  (Audio|Components|Audio|Play (Variables|Default|GetBGM) 0.0))

(event EventBeginPlay
  (CallFunction|Init)
  (CallFunction|PlayBGM)
  (bind _asplayer_bp (Utilities|Casting|CastToPlayer_BP (Game|Player|GetPlayerPawn 0)))
  (EventDispatchers|BindEventtoStopBGM _asplayer_bp (delegate Custom|StopBGM))
  (bind _asgame_mode_bp (Utilities|Casting|CastToGameMode_BP (Game|GetGameMode)))
  (EventDispatchers|BindEventtoOnRespawn _asgame_mode_bp (delegate Custom|PlayBGM)))

(event Collision|EventActorBeginOverlap
  (params (OtherActor :type Actor%20Object%20Reference)))

(event EventTick
  (params (DeltaSeconds :type Float%20%28single-precision%29)))

(fn ConstructionScript)

(fn Init
  (bind _returnvalue (Game|GetCurrentLevelName true))
  (Variables|Default|SetCurrentLevelName _returnvalue)
  (switch string _returnvalue
    (:Stage1_1
      (Variables|Default|SetBGM (Variables|Default|GetBGM_Stage1_1_Cue)))
    (:Stage1_2
      (Variables|Default|SetBGM (Variables|Default|GetBGM_Stage1_2_Cue)))
    (:Stage1_3
      (Variables|Default|SetBGM (Variables|Default|GetBGM_Stage1_3_Cue)))
    (:Stage2_1
      (Variables|Default|SetBGM (Variables|Default|GetBGM_Stage2_1_Cue)))
    (:Stage2_2
      (Variables|Default|SetBGM (Variables|Default|GetBGM_Stage2_2_Cue)))
    (:Stage2_3
      (Variables|Default|SetBGM (Variables|Default|GetBGM_Stage2_3_Cue)))))