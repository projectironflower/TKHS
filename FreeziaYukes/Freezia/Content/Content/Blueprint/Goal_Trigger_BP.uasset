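; Goal trigger that ends a stage when Player_BP enters its box and handles the transitions out of it.
; Overlap clears the player, stops the BGM, fires CallOnPlayer and stream-loads NextLevel hidden, then sets LoadFinished.
; ChangeToNextScene waits on that flag, which SetNextLevelName also sets, while Title and StageSelect exits are ungated.
; All three exits spawn SmoleFade_BP, blend the view to the player and fade the camera before opening the level.
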(event OnComponentBeginOverlap(Box)
  (params (OverlappedComponent :type Primitive%20Component%20Object%20Reference) (OtherActor :type Actor%20Object%20Reference) (OtherComp :type Primitive%20Component%20Object%20Reference) (OtherBodyIndex :type Integer) (bFromSweep :type Boolean) (SweepResult :type Hit%20Result%20Structure%20%28by%20ref%29))
  (bind _asplayer_bp (Utilities|Casting|CastToPlayer_BP OtherActor))
  (Default|OnClear _asplayer_bp)
  (bind _returnvalue (Actor|GetActorOfClass "/Game/Content/Blueprint/BGMPlayer_BP.BGMPlayer_BP_C"))
  (Default|StopBGM _returnvalue)
  (Default|CallOnPlayer)
  (Game|LoadStreamLevel(byName) (Variables|Default|GetNextLevel) false)
  (Variables|Default|SetLoadFinished true))

(event Custom|ChangeToNextScene
  (if (Variables|Default|GetLoadFinished)
    (bind _returnvalue (Game|SpawnActorfromClass "/Game/Content/Blueprint/SmoleFade_BP.SmoleFade_BP_C" (Math|Transform|MakeTransform (+ (Transformation|GetActorLocation (Game|Player|GetPlayerPawn 0)) "0, 0,-200.000000")) "Undefined" 0 0))
    (Default|Fadein _returnvalue)
    (Game|Player|SetViewTargetwithBlend (Game|GetPlayerController 0) (Game|Player|GetPlayerPawn 0) 1.5 "VTBlend_Cubic" 0.0 false)
    (Utilities|FlowControl|Delay 2.0)
    (CameraFades|StartCameraFade (Game|GetPlayerCameraManager 0) 0.0 1.0 1.0 "(R=1.000000,G=1.000000,B=1.000000,A=1.000000)" false true)
    (Utilities|FlowControl|Delay 1.0)
    (Game|OpenLevel(byName) (Variables|Default|GetNextLevel))))

(event Custom|ChangeToStageSelect
  (bind _returnvalue (Game|SpawnActorfromClass "/Game/Content/Blueprint/SmoleFade_BP.SmoleFade_BP_C" (Math|Transform|MakeTransform (+ (Transformation|GetActorLocation (Game|Player|GetPlayerPawn 0)) "0, 0,-200.000000")) "Undefined" 0 0))
  (Default|Fadein _returnvalue)
  (Game|Player|SetViewTargetwithBlend (Game|GetPlayerController 0) (Game|Player|GetPlayerPawn 0) 1.5 "VTBlend_Cubic" 0.0 false)
  (Utilities|FlowControl|Delay 2.0)
  (CameraFades|StartCameraFade (Game|GetPlayerCameraManager 0) 0.0 1.0 1.0 "(R=1.000000,G=1.000000,B=1.000000,A=1.000000)" false true)
  (Utilities|FlowControl|Delay 1.0)
  (Game|OpenLevel(byName) "StageSelect"))

(event Custom|SetNextLevelName
  (params (NextLevel :type Name))
  (Variables|Default|SetLoadFinished true)
  (Variables|Default|SetNextLevel NextLevel))

(event Custom|ChangeToTitle
  (bind _returnvalue (Game|SpawnActorfromClass "/Game/Content/Blueprint/SmoleFade_BP.SmoleFade_BP_C" (Math|Transform|MakeTransform (+ (Transformation|GetActorLocation (Game|Player|GetPlayerPawn 0)) "0, 0,-200.000000")) "Undefined" 0 0))
  (Default|Fadein _returnvalue)
  (Game|Player|SetViewTargetwithBlend (Game|GetPlayerController 0) (Game|Player|GetPlayerPawn 0) 1.5 "VTBlend_Cubic" 0.0 false)
  (Utilities|FlowControl|Delay 2.0)
  (CameraFades|StartCameraFade (Game|GetPlayerCameraManager 0) 0.0 1.0 1.0 "(R=1.000000,G=1.000000,B=1.000000,A=1.000000)" false true)
  (Utilities|FlowControl|Delay 1.0)
  (Game|OpenLevel(byName) "Title"))

(event EventBeginPlay)

(event Collision|EventActorBeginOverlap
  (params (OtherActor :type Actor%20Object%20Reference)))

(event EventTick
  (params (DeltaSeconds :type Float%20%28single-precision%29)))

(fn ConstructionScript)