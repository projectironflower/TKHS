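; Death mist actor that carries the camera from where it spawns back to the respawn point at the player start.
; Construction reads the target from GameMode_BP and scales speed with distance, with a minimum, capping travel at about five seconds.
; BeginPlay copies the player's spring arm scale and blends the view to itself.
; Tick moves it straight without sweep; on arrival it destroys the player pawn, then itself.
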(event EventBeginPlay
  (bind _asplayer_bp (Utilities|Casting|CastToPlayer_BP (Game|Player|GetPlayerPawn 0)))
  (Transformation|SetWorldScale3D (Variables|Default|GetSpringArm) (Transformation|GetWorldScale (Variables|/Game/Content/Blueprint/Player/Player_BP.Player_BP_C|GetSpringArm _asplayer_bp)))
  (Utilities|FlowControl|Delay 0.2)
  (Game|Player|SetViewTargetwithBlend (Game|GetPlayerController 0) self 1.0 "VTBlend_Linear" 0.0 false))

(event Collision|EventActorBeginOverlap
  (params (OtherActor :type Actor%20Object%20Reference)))

(event EventTick
  (params (DeltaSeconds :type Float%20%28single-precision%29))
  (bind _returnvalue (Transformation|GetActorLocation))
  (bind _playerstart (Variables|Default|GetPlayerStart))
  (bind _respawnoffset (Variables|Default|GetRespawnOffset))
  (bind _returnvalue_2 (Transformation|GetActorLocation _playerstart))
  (bind _returnvalue_3 (+ _returnvalue_2 _respawnoffset))
  (bind _returnvalue_4 (- _returnvalue_3 _returnvalue))
  (bind _returnvalue_5 (Math|Vector|VectorLength _returnvalue_4))
  (if (>= _returnvalue_5 15.0)
    (Transformation|SetActorLocation (+ _returnvalue (* (/ _returnvalue_4 _returnvalue_5) (* DeltaSeconds (Variables|Default|GetMoveSpeed)))) false false)
    (else
      (Utilities|FlowControl|DoOnce false
        (:Completed
          (Actor|DestroyActor (Game|Player|GetPlayerPawn 0))
          (Utilities|FlowControl|Delay 0.2)
          (Actor|DestroyActor))))))

(fn ConstructionScript
  (bind _asgame_mode_bp (Utilities|Casting|CastToGameMode_BP (Game|GetGameMode)))
  (Variables|Default|SetRespawnOffset (Variables|/Game/Content/Blueprint/GameMode_BP.GameMode_BP_C|GetRespawnOffset _asgame_mode_bp))
  (bind _output_get (Variables|Default|SetPlayerStart (Variables|/Game/Content/Blueprint/GameMode_BP.GameMode_BP_C|GetPlayerStart _asgame_mode_bp)))
  (Variables|Default|SetMoveSpeed (Math|Float|Max(Float) (* (Math|Vector|VectorLength (- (+ (Transformation|GetActorLocation _output_get) (Variables|Default|GetRespawnOffset)) (Transformation|GetActorLocation))) 0.2) 2e+02)))