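; A water surface hazard that kills the player on contact unless it is frozen.
; A Box overlap deals the player's MaxLife as damage through Player_BP's Damage while IsFreezed is false.
; The Freeze function sets that flag and swaps the mesh material between ice shards and water splash, turning the lethal check on or off.
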(event OnComponentBeginOverlap(Box)
  (params (OverlappedComponent :type Primitive%20Component%20Object%20Reference) (OtherActor :type Actor%20Object%20Reference) (OtherComp :type Primitive%20Component%20Object%20Reference) (OtherBodyIndex :type Integer) (bFromSweep :type Boolean) (SweepResult :type Hit%20Result%20Structure%20%28by%20ref%29))
  (bind (_asplayer_bp _bsuccess) (Utilities|Casting|CastToPlayer_BP OtherActor))
  (if (not (Variables|Default|GetIsFreezed))
    (if _bsuccess
      (Default|Damage _asplayer_bp (Variables|/Game/Content/Blueprint/Player/Player_BP.Player_BP_C|GetMaxLife _asplayer_bp)))))

(event EventBeginPlay)

(event Collision|EventActorBeginOverlap
  (params (OtherActor :type Actor%20Object%20Reference)))

(event EventTick
  (params (DeltaSeconds :type Float%20%28single-precision%29)))

(fn ConstructionScript)

(fn Freeze
  (params (freeze :type Boolean))
  (bind _staticmeshcomponent (Variables|Debug|GetStaticMeshComponent))
  (bind _output_get (Variables|Default|SetIsFreezed freeze))
  (if _output_get
    (Rendering|Material|SetMaterial _staticmeshcomponent 0 "/Game/Content/Blueprint/Material/T_IceShards_E_Mat.T_IceShards_E_Mat")
    (else
      (Rendering|Material|SetMaterial _staticmeshcomponent 0 "/Game/mogu_sample/new/material/MI_SplashBase.MI_SplashBase"))))