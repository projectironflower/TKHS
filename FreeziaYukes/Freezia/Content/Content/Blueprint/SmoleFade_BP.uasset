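; Smoke fade effect actor that grows or shrinks two smoke components, one for the player and one for the camera.
; BeginPlay starts both at small scale; FadeIn and FadeOut set a flag and move them near the player pawn's mesh and camera.
; Tick multiplies their scale each frame while a flag is set, so speed is frame-rate dependent.
; Neither flag is cleared in these graphs.
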(event Custom|FadeIn
  (Variables|Default|SetIsFadeIn true)
  (bind _asplayer_bp (Utilities|Casting|CastToPlayer_BP (Game|Player|GetPlayerPawn 0)))
  (Transformation|SetWorldLocation (Variables|Default|GetPlayerSmoke) (+ (Transformation|GetWorldLocation (Variables|/Script/Engine.Character|GetMesh _asplayer_bp)) "-50.000000, 0, 0") false false)
  (Transformation|SetWorldLocation (Variables|Default|GetCameraSmoke) (+ (Transformation|GetWorldLocation (Variables|/Game/Content/Blueprint/Player/Player_BP.Player_BP_C|GetCamera _asplayer_bp)) "20.000000,0.000000,-100.000000") false false))

(event Custom|FadeOut
  (Variables|Default|SetIsFadeOut true)
  (bind _asplayer_bp (Utilities|Casting|CastToPlayer_BP (Game|Player|GetPlayerPawn 0)))
  (Transformation|SetWorldLocation (Variables|Default|GetPlayerSmoke) (+ (Transformation|GetWorldLocation (Variables|/Script/Engine.Character|GetMesh _asplayer_bp)) "-50.000000, 0, 0") false false)
  (Transformation|SetWorldLocation (Variables|Default|GetCameraSmoke) (+ (Transformation|GetWorldLocation (Variables|/Game/Content/Blueprint/Player/Player_BP.Player_BP_C|GetCamera _asplayer_bp)) "20.000000,0.000000,-100.000000") false false))

(event EventBeginPlay
  (Transformation|SetWorldScale3D (Variables|Default|GetPlayerSmoke) "0.100000,0.100000,0.100000"))

(event Collision|EventActorBeginOverlap
  (params (OtherActor :type Actor%20Object%20Reference)))

(event EventTick
  (params (DeltaSeconds :type Float%20%28single-precision%29))
  (bind _playersmoke (Variables|Default|GetPlayerSmoke))
  (bind _camerasmoke (Variables|Default|GetCameraSmoke))
  (bind _returnvalue (Transformation|GetWorldScale _playersmoke))
  (bind _returnvalue_2 (Transformation|GetWorldScale _camerasmoke))
  (Utilities|FlowControl|Sequence
    (:then_0
      (if (Variables|Default|GetIsFadeIn)
        (Transformation|SetWorldScale3D _playersmoke (* _returnvalue 1.025))
        (Transformation|SetWorldScale3D _camerasmoke (* _returnvalue_2 1.01))))
    (:then_1
      (if (Variables|Default|GetIsFadeOut)
        (Transformation|SetWorldScale3D _playersmoke (* _returnvalue 0.975))
        (Transformation|SetWorldScale3D _camerasmoke (* _returnvalue_2 0.99))))))

(fn ConstructionScript)