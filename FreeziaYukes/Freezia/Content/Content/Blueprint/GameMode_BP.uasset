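; Game mode that respawns the player whenever the pawn is destroyed and tracks checkpoint progress.
; It binds to the pawn's destroyed event, then spawns a new Player_BP at the player start plus a respawn offset, calls its Respawn and possesses it.
; After possession it switches the view to the camera tagged DeathCamera and rebinds the event.
; SetRespawnOffset updates the offset only for higher-numbered checkpoints.
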(event Custom|RespawnPlayer
  (params (DestroyedActor :type Actor%20Object%20Reference))
  (bind _returnvalue (Class|GameModeBase|FindPlayerStart))
  (bind _returnvalue_2 (Transformation|GetActorTransform _returnvalue))
  (bind (_location _rotation _scale) (Math|Transform|BreakTransform _returnvalue_2))
  (bind _returnvalue_3 (Game|SpawnActorfromClass "/Game/Content/Blueprint/Player/Player_BP.Player_BP_C" (Math|Transform|MakeTransform (+ _location (Variables|Default|GetRespawnOffset)) _rotation _scale) "Undefined" 0 0))
  (Utilities|FlowControl|Delay 0.01)
  (Default|Respawn _returnvalue_3)
  (Pawn|Possess (Game|GetPlayerController 0) _returnvalue_3)
  (Utilities|SetDeathCamera
    (:Completed
      (Utilities|FlowControl|Delay 0.2)
      (Game|BindEventtoOnDestroyed _returnvalue_3 (delegate Custom|RespawnPlayer)))))

(event Custom|SetRespawnOffset
  (params (Location :type Vector) (CheckPointNum :type Integer))
  (if (> CheckPointNum (Variables|Default|GetCheckPointNum))
    (Variables|Default|SetRespawnOffset Location)
    (Variables|Default|SetCheckPointNum CheckPointNum)))

(event EventBeginPlay
  (Game|BindEventtoOnDestroyed (Game|Player|GetPlayerPawn 0) (delegate Custom|RespawnPlayer))
  (bind _asplayer_start (Utilities|Casting|CastToPlayerStart (Class|GameModeBase|FindPlayerStart)))
  (Variables|Default|SetPlayerStart _asplayer_start))

(event EventTick
  (params (DeltaSeconds :type Float%20%28single-precision%29)))

(fn ConstructionScript)