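; Puzzle block the player can grab and drag, which falls when unsupported and slides along frozen WaterBlock_BP ice.
; Each Tick, overlap boxes check ground, sides and ice, then drive falling, following the player at a stored offset, or sliding.
; Release snaps Y to a 100-unit grid, landing snaps Z to 50, and falling or reaching ice while pushed or pulled releases the player.
; Respawn events and death volumes restore its starting position.
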(event Custom|Reset
  (Transformation|SetActorLocation (Variables|Default|GetBasePosition) false false))

(event EventBeginPlay
  (bind _returnvalue (Transformation|GetActorLocation))
  (bind (_x _y _z) (Math|Vector|BreakVector _returnvalue))
  (Variables|Default|SetBasePositionZ _z)
  (Variables|Default|SetOffIceY (- _y 1e+02))
  (Variables|Default|SetBasePosition (Transformation|GetActorLocation))
  (bind _asgame_mode_bp (Utilities|Casting|CastToGameMode_BP (Game|GetGameMode)))
  (EventDispatchers|BindEventtoOnRespawn _asgame_mode_bp (delegate Custom|Reset)))

(event Collision|EventActorBeginOverlap
  (params (OtherActor :type Actor%20Object%20Reference))
  (Utilities|Casting|CastToDeathTriggerVolume_BP OtherActor)
  (CallFunction|Reset))

(event EventTick
  (params (DeltaSeconds :type Float%20%28single-precision%29))
  (bind _returnvalue (Transformation|GetActorLocation))
  (bind (_x _y _z) (Math|Vector|BreakVector _returnvalue))
  (Utilities|FlowControl|Sequence
    (:then_0
      (Variables|Default|SetCanMoveRight true)
      (Variables|Default|SetCanMoveLeft true)
      (Variables|Default|SetIsFalling true))
    (:then_1
      (CallFunction|CheckBottom)
      (if (Variables|Default|GetIsFalling)
        (Utilities|FlowControl|DoOnce false :!label _label
          (:Completed
            (bind _asplayer_bp (Utilities|Casting|CastToPlayer_BP (Game|Player|GetPlayerPawn 0)))
            (Default|Release _asplayer_bp)))
        (else
          (goto _label Reset))))
    (:then_2
      (CallFunction|Fall))
    (:then_3
      (Utilities|CheckRight))
    (:then_4
      (Utilities|CheckLeft))
    (:then_5
      (Utilities|CheckIce))
    (:then_6
      (if (not (Variables|Default|GetIsFalling))
        (if (Variables|Default|GetisGrabbed)
          (bind _asplayer_bp_2 (Utilities|Casting|CastToPlayer_BP (Game|Player|GetPlayerPawn 0)))
          (Transformation|SetActorLocation (Math|Vector|MakeVector (.X (Math|Vector|BreakVector (+ (Transformation|GetActorLocation _asplayer_bp_2) (Variables|Default|GetOffsetFromPlayer)))) (.Y (Math|Vector|BreakVector (+ (Transformation|GetActorLocation _asplayer_bp_2) (Variables|Default|GetOffsetFromPlayer)))) (Variables|Default|GetBasePositionZ)) false false)
          (CallFunction|CheckSide)
          (elif (Variables|Default|GetIsOnIce)
            (Transformation|SetActorLocation (Math|Vector|MakeVector _x (+ _y (* (Variables|Default|GetToRight) 5.0)) _z) false false)
            (elif (> (Variables|Default|GetToRight) 0.0)
              (if (< (.Y (Math|Vector|BreakVector (Transformation|GetActorLocation))) (+ (Variables|Default|GetOffIceY) 1e+02))
                (Transformation|SetActorLocation (Math|Vector|MakeVector _x (+ _y (* (Variables|Default|GetToRight) 5.0)) _z) false false)
                (else
                  (Variables|Default|SetToRight 0.0)))
              (elif (< (Variables|Default|GetToRight) 0.0)
                (if (> (.Y (Math|Vector|BreakVector (Transformation|GetActorLocation))) (- (Variables|Default|GetOffIceY) 1e+02))
                  (Transformation|SetActorLocation (Math|Vector|MakeVector _x (+ _y (* (Variables|Default|GetToRight) 5.0)) _z) false false)
                  (else
                    (Variables|Default|SetToRight 0.0)))))))))))

(fn ConstructionScript)

(fn Move
  (params (DeltaSecond :type Float%20%28single-precision%29) (Player :type Player%20BP%20Object%20Reference))
  (Transformation|SetActorLocation (+ (* (Math|Vector|GetRightVector (Variables|/Script/Engine.Character|GetMesh Player)) (* (Variables|Default|GetMoveSpeed) (* DeltaSecond 6e+01) (Variables|/Game/Content/Blueprint/Player/Player_BP.Player_BP_C|GetAxisForword Player))) (Transformation|GetActorLocation)) false false))

(fn Grab
  (bind _asplayer_bp (Utilities|Casting|CastToPlayer_BP (Game|Player|GetPlayerPawn 0)))
  (if (Utilities|CanGrab _asplayer_bp)
    (Collision|SetCollisionEnabled (Variables|Default|GetStaticMesh) "NoCollision")
    (Variables|Default|SetisGrabbed true)
    (Variables|Default|SetOffsetFromPlayer (- (Transformation|GetActorLocation) (Transformation|GetActorLocation _asplayer_bp)))
    (return true)
    (else
      (return false))))

(fn Release
  (bind _returnvalue (Transformation|GetActorLocation))
  (bind (_x _y _z) (Math|Vector|BreakVector _returnvalue))
  (bind (_x_2 _y_2 _z_2) (Math|Vector|BreakVector _returnvalue))
  (bind _returnvalue_2 (+ _y 7e+01))
  (bind _returnvalue_3 (+ _y_2 3e+01))
  (Collision|SetCollisionEnabled (Variables|Default|GetStaticMesh) "QueryAndPhysics")
  (Variables|Default|SetisGrabbed false)
  (if (> (.Y (Math|Vector|BreakVector (Variables|Default|GetOffsetFromPlayer))) 0.0)
    (Transformation|SetActorLocation (Math|Vector|MakeVector _x (- _returnvalue_2 (Math|Float|%(Float) _returnvalue_2 1e+02)) _z) false false)
    (else
      (Transformation|SetActorLocation (Math|Vector|MakeVector _x_2 (- _returnvalue_3 (Math|Float|%(Float) _returnvalue_3 1e+02)) _z_2) false false))))

(fn Fall
  (bind _returnvalue (Transformation|GetActorLocation))
  (bind (_x _y _z) (Math|Vector|BreakVector _returnvalue))
  (if (Variables|Default|GetIsFalling)
    (Transformation|SetActorLocation (Math|Vector|MakeVector _x _y (- _z (Variables|Default|GetFallSpeed))) false false)
    (Collision|SetCollisionEnabled (Variables|Default|GetStaticMesh) "QueryAndPhysics")
    (Variables|Default|SetisGrabbed false)))

(fn CheckBottom
  (bind _returnvalue (Transformation|GetActorLocation))
  (bind (_x _y _z) (Math|Vector|BreakVector _returnvalue))
  (for _array_element (Class|PrimitiveComponent|GetOverlappingComponents (Variables|Default|GetBottomBox))
    (if (Class|PrimitiveComponent|CanCharacterStepUp _array_element (Game|Player|GetPlayerPawn 0))
      (Variables|Default|SetIsFalling false)
      (Transformation|SetActorLocation (Math|Vector|MakeVector _x _y (- _z (Math|Float|%(Float) _z 5e+01))) false false)
      (Variables|Default|SetBasePositionZ (+ _z 0.0)))))

(fn CheckSide
  (bind _asplayer_bp (Utilities|Casting|CastToPlayer_BP (Utilities|Array|Get(acopy) (Collision|GetOverlappingActors (Variables|Default|GetRightBox) "/Game/Content/Blueprint/Player/Player_BP.Player_BP_C" :!class /Script/Engine.PrimitiveComponent)))
    (:then
      (Transformation|SetActorLocation _asplayer_bp (+ (Transformation|GetActorLocation _asplayer_bp) (* "0,100.000000, 0" (Utilities|Time|GetWorldDeltaSeconds))) false false)
      (Variables|Default|SetOffsetFromPlayer (+ (Variables|Default|GetOffsetFromPlayer) (* "0,-100.000000, 0" (Utilities|Time|GetWorldDeltaSeconds)))))
    (:CastFailed
      (bind _asplayer_bp_2 (Utilities|Casting|CastToPlayer_BP (Utilities|Array|Get(acopy) (Collision|GetOverlappingActors (Variables|Default|GetLeftBox) "/Game/Content/Blueprint/Player/Player_BP.Player_BP_C" :!class /Script/Engine.PrimitiveComponent))))
      (Transformation|SetActorLocation _asplayer_bp_2 (+ (Transformation|GetActorLocation _asplayer_bp_2) (* "0,-100.000000, 0" (Utilities|Time|GetWorldDeltaSeconds))) false false)
      (Variables|Default|SetOffsetFromPlayer (+ (Variables|Default|GetOffsetFromPlayer) (* "0,100.000000, 0" (Utilities|Time|GetWorldDeltaSeconds)))))))

(fn CheckonIce
  (for _array_element (Class|PrimitiveComponent|GetOverlappingComponents (Variables|Default|GetBottomBox))
    (if (Components|ComponentHasTag _array_element "DamageArea")
      (bind _aswater_block_bp (Utilities|Casting|CastToWaterBlock_BP (Components|GetOwner _array_element)))
      (return (Variables|/Game/Content/Blueprint/WaterBlock_BP.WaterBlock_BP_C|GetIsFreezed _aswater_block_bp) (not (Variables|/Game/Content/Blueprint/WaterBlock_BP.WaterBlock_BP_C|GetIsFreezed _aswater_block_bp)))))
  (return false false))