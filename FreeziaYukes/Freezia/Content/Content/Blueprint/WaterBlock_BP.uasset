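; WaterBlock_BP is a water hazard block that damages the player by their full MaxLife when they enter its DamageArea, unless the block is frozen.
; Freeze sets the frozen state, swaps the Water mesh between lake and ice materials, and calls itself on water blocks overlapping its ContactBox.
; The state change thus flood-fills through connected blocks, with an unchanged-state check ending the recursion.
; The construction script applies IsVisible to the Water mesh.
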(event OnComponentBeginOverlap(DamageArea)
  (params (OverlappedComponent :type Primitive%20Component%20Object%20Reference) (OtherActor :type Actor%20Object%20Reference) (OtherComp :type Primitive%20Component%20Object%20Reference) (OtherBodyIndex :type Integer) (bFromSweep :type Boolean) (SweepResult :type Hit%20Result%20Structure%20%28by%20ref%29))
  (bind _asplayer_bp (Utilities|Casting|CastToPlayer_BP OtherActor))
  (if (not (Variables|Default|GetIsFreezed))
    (Default|Damage _asplayer_bp (Variables|/Game/Content/Blueprint/Player/Player_BP.Player_BP_C|GetMaxLife _asplayer_bp))))

(event EventBeginPlay)

(event Collision|EventActorBeginOverlap
  (params (OtherActor :type Actor%20Object%20Reference)))

(event EventTick
  (params (DeltaSeconds :type Float%20%28single-precision%29)))

(fn ConstructionScript
  (Rendering|SetVisibility (Variables|Default|GetWater) (Variables|Default|GetIsVisible) false))

(fn Freeze
  (params (Freeze :type Boolean))
  (bind _water (Variables|Default|GetWater))
  (if (Math|Boolean|NotEqual(Boolean) Freeze (Variables|Default|GetIsFreezed))
    (bind _output_get (Variables|Default|SetIsFreezed Freeze))
    (if _output_get
      (Rendering|Material|SetMaterial _water 0 "/Game/Content/Blueprint/Material/T_IceShards_E_Mat.T_IceShards_E_Mat")
      (else
        (Rendering|Material|SetMaterial _water 0 "/Game/StarterContent/Materials/M_Water_Lake.M_Water_Lake")))
    (for _array_element (Collision|GetOverlappingActors (Variables|Default|GetContactBox) "WaterBlock_BP_C" :!class /Script/Engine.PrimitiveComponent)
      (if (.bSuccess (Utilities|Casting|CastToWaterBlock_BP _array_element))
        (CallFunction|Freeze (.AsWater%20Block%20BP (Utilities|Casting|CastToWaterBlock_BP _array_element)) _output_get)))
    (return)
    (else
      (return))))